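; Continuous beam projectile actor that draws a particle beam from the player character's arrow to its target location.
; Proj_PT_Set assigns the fire, beam, explosion and beam-end templates, then attaches the actor to the player.
; Tick polls ThirdPersonCharacter_Fix to update beam endpoints, showing the explosion on targeted hits or the end effect otherwise.
; When the character's BeamContinue turns false, it deactivates the particles and destroys itself after a short delay.
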(event `self.ReceiveTick`
  (params (DeltaSeconds :type "Float (single-precision)"))
  (bind _returnvalue (`self.K2_GetActorLocation`))
  (bind _projexp_pt (`self.ProjExp_PT`))
  (bind _targetlocation (`self.TargetLocation`))
  (bind _proj_pt (`self.Proj_PT`))
  (bind _projbeamend_pt (`self.ProjBeamEnd_PT`))
  ;[1 1 1] Continuous Beam
  (bind _asthird_person_character_fix (cast `/Game/M5VFXRPG2/Blueprint/ThirdPersonCharacter_Fix` (`GameplayStatics.GetPlayerCharacter` 0)))
  (set `self.TargetLocation` (`/Game/M5VFXRPG2/Blueprint/ThirdPersonCharacter_Fix.TargetHitLocation` _asthird_person_character_fix))
  (bind _arrow1 (`/Game/M5VFXRPG2/Blueprint/ThirdPersonCharacter_Fix.Arrow1` _asthird_person_character_fix))
  (set `self.SourceLocation` (`SceneComponent.K2_GetComponentLocation` _arrow1))
  (set `self.Impactnormal` (`KismetMathLibrary.Conv_VectorToRotator` (`/Game/M5VFXRPG2/Blueprint/ThirdPersonCharacter_Fix.Impactnormal` _asthird_person_character_fix)))
  (`SceneComponent.K2_SetWorldRotation` (`self.ProjFire_PT`) (`SceneComponent.K2_GetComponentRotation` _arrow1) false false)
  (`SceneComponent.K2_SetWorldRotation` (`self.Sphere`) (`KismetMathLibrary.FindLookAtRotation` _returnvalue (+ _returnvalue (0.0 0.0 0.0))) false false)
  (bind _asthird_person_character_fix_2 (cast `/Game/M5VFXRPG2/Blueprint/ThirdPersonCharacter_Fix` (`GameplayStatics.GetPlayerCharacter` 0)))
  (bind _output_get (set `self.beamcontinue` (`/Game/M5VFXRPG2/Blueprint/ThirdPersonCharacter_Fix.beamContinue` _asthird_person_character_fix_2)))
  (if _output_get
    (for _index (range 11)
      (`ParticleSystemComponent.SetBeamSourcePoint` _proj_pt _index (`self.SourceLocation`) 0)
      (`ParticleSystemComponent.SetBeamTargetPoint` _proj_pt _index _targetlocation 0)
      (if (`/Game/M5VFXRPG2/Blueprint/ThirdPersonCharacter_Fix.Targeted` _asthird_person_character_fix_2)
        (`ActorComponent.Activate` _projexp_pt false)
        (`SceneComponent.K2_SetWorldRotation` _projexp_pt (`self.Impactnormal`) false false)
        (`SceneComponent.K2_SetWorldLocation` _projexp_pt _targetlocation false false)
        (`KismetSystemLibrary.Delay` 0.0)
        (`ActorComponent.Deactivate` _projbeamend_pt)
        (else
          (`ActorComponent.Activate` _projbeamend_pt false)
          (`|ExecutionSequence`
            (:`then_0`
              (`SceneComponent.K2_SetWorldLocation` _projbeamend_pt _targetlocation false false)
              (`KismetSystemLibrary.Delay` 0.0)
              (`ActorComponent.Deactivate` _projexp_pt))
            (:`then_1`
              (`KismetSystemLibrary.Delay` 0.5)
              (`KismetSystemLibrary.PrintString` "none Target" true true (struct :`R` 1.0 :`A` 1.0) 0.5))))))
    (else
      (`ActorComponent.Deactivate` _proj_pt)
      (`self.SetLifeSpan` 2.0)
      (`ActorComponent.Deactivate` (`self.ProjFire_PT`))
      (`ActorComponent.Deactivate` (`self.Proj_PT`))
      (`ActorComponent.Deactivate` (`self.ProjBeamEnd_PT`))
      (`ActorComponent.Deactivate` (`self.ProjExp_PT`))
      (`KismetSystemLibrary.Delay` 2.0)
      (`self.K2_DestroyActor`))))

(event `Proj_PT_Set`
  (params (ProjectileFire_PT :type "ParticleSystem Object Reference") (projectile_PT :type "ParticleSystem Object Reference") (ProjectileExplosion_PT :type "ParticleSystem Object Reference") (ProjectileBeamEnd_PT :type "ParticleSystem Object Reference") (TargetPoint :type "Vector Structure") (IsTargetObject :type Boolean) (NoneTargetPoint :type "Vector Structure") (beamContinue :type Boolean))
  (bind _projexp_pt (`self.ProjExp_PT`))
  ;[1 1 1] Projectile Particle
  (bind _output_get (set `self.beamcontinue` beamContinue))
  (if _output_get
    (set `self.TargetLocation` TargetPoint)
    (else
      (set `self.TargetLocation` NoneTargetPoint)))
  (`ParticleSystemComponent.SetTemplate` (`self.ProjFire_PT`) ProjectileFire_PT)
  (`ActorComponent.Deactivate` _projexp_pt)
  (`ActorComponent.Deactivate` (`self.ProjBeamEnd_PT`))
  (`ParticleSystemComponent.SetTemplate` _projexp_pt ProjectileExplosion_PT)
  (`ParticleSystemComponent.SetTemplate` (`self.ProjBeamEnd_PT`) ProjectileBeamEnd_PT)
  (bind _asthird_person_character_fix (cast `/Game/M5VFXRPG2/Blueprint/ThirdPersonCharacter_Fix` (`GameplayStatics.GetPlayerCharacter` 0)))
  (`self.K2_AttachToActor` self (`ActorComponent.GetOwner` (`/Game/M5VFXRPG2/Blueprint/ThirdPersonCharacter_Fix.Arrow1` _asthird_person_character_fix)) "None" "KeepWorld" "KeepWorld" "KeepWorld" true)
  (`ParticleSystemComponent.SetTemplate` (`self.Proj_PT`) projectile_PT)
  (for _index (range 2)
    (`ParticleSystemComponent.SetBeamSourcePoint` (`self.Proj_PT`) _index (`self.SourceLocation`) 0)
    (`ParticleSystemComponent.SetBeamTargetPoint` (`self.Proj_PT`) _index (`self.TargetLocation`) 0)
    (if (`self.beamcontinue`)
      _
      (else
        _))
    (`self.SetLifeSpan` 0.0)))

(fn `UserConstructionScript`)
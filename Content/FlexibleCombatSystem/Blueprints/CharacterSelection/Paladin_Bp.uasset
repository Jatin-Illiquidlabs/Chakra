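; Playable Paladin character with four input-driven abilities: sword teleport, self-heal, a ground-targeted ability and a charge ultimate.
; Targeted abilities set a type and hand cursor, then Select caches the cursor location, walks into range if needed and casts, with DoOnce gates blocking repeats.
; Pressing Ability1 again while targeting teleports to the BP_TeleportSword actor.
; The ultimate lerps a swept move toward the enemy via timeline, applying sphere-trace damage on a blocking hit.
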(event `self.ReceiveBeginPlay`
  (`self.PlayAnimMontage` "/Game/FlexibleCombatSystem/NewAnims/Montages/PaladinStart.PaladinStart"))

(event `self.ReceiveTick`
  (params (DeltaSeconds :type "Float (single-precision)"))
  (`parent.ReceiveTick` DeltaSeconds))

(event `InputAction|CancelAbility`
  (params (Key :type "Key Structure"))
  ;[1 0 0] Cancel
  (:`Pressed`
    (if (`self.SelecetedPoint`)
      (set `self.SelecetedPoint` false)
      (set `PlayerController.CurrentMouseCursor` "Default" (`GameplayStatics.GetPlayerController` 0))
      (set `self.AbleToAttack` true))))

(event `InputAction|Ability1`
  (params (Key :type "Key Structure"))
  ;[1 1 1] Ability1
  (:`Pressed`
    (if (`self.SelecetedPoint`)
      (bind _returnvalue (`GameplayStatics.GetActorOfClass` "/Game/FlexibleCombatSystem/Blueprints/Weapons/PaladinAbility/BP_TeleportSword.BP_TeleportSword_C"))
      (if (`/Game/FlexibleCombatSystem/Blueprints/Weapons/PaladinAbility/BP_TeleportSword.Located` _returnvalue)
        (bind _returnvalue_2 (`self.K2_GetActorLocation` _returnvalue))
        (`self.K2_TeleportTo` _returnvalue_2)
        (`NiagaraFunctionLibrary.SpawnSystemAtLocation` "/Game/Plugins/DarkSocerer_Animset/demo/FX/NS_FireToon.NS_FireToon" _returnvalue_2)
        (set `self.SelecetedPoint` false)
        (`self.K2_DestroyActor` _returnvalue))
      (else
        (`self.StopMovementController`)
        (set `self.SelecetedPoint` true)
        (set `self.AbilityType` "NewEnumerator0")
        (set `PlayerController.CurrentMouseCursor` "Hand" (`GameplayStatics.GetPlayerController` 0))))))

(event `InputAction|Select`
  (params (Key :type "Key Structure"))
  (bind _enemylocaiton (`self.EnemyLocaiton`))
  (bind _radialforce (`self.RadialForce`))
  (bind _mesh (`self.Mesh`))
  (bind _returnvalue (`KismetMathLibrary.Vector_Distance` (`self.CachedDestination`) (`self.K2_GetActorLocation`)))
  (bind _returnvalue_2 (`KismetMathLibrary.Vector_Distance` (`self.CachedDestination`) (`self.K2_GetActorLocation`)))
  (bind _returnvalue_3 (`KismetMathLibrary.Vector_Distance` (`self.CachedDestination`) (`self.K2_GetActorLocation`)))
  ;[0.8785 1 0] Selection
  (:`Pressed`
    (if (`self.SelecetedPoint`)
      (bind _output_get (set `self.CachedDestination` (`.Location` (`self.GetLocationUnderCursor`))))
      (switch `/Game/FlexibleCombatSystem/Blueprints/PaladinChar_AbilityType` (`self.AbilityType`)
        (:`NewEnumerator0`
          (`/Engine/EditorBlueprintResources/StandardMacros.DoOnce` false :!label _label
            (:`Completed`
              (set `self.AbleToAttack` false)
              (set `self.TargetDistance` _returnvalue_3)
              (if (not (<= _returnvalue_3 1200.0))
                (`self.Out Range Move` 600.0)
                (`KismetSystemLibrary.Delay` 2.0))
              (`self.PlayAnimMontage` "/Game/FlexibleCombatSystem/NewAnims/Montages/TeleportAttack_Montage.TeleportAttack_Montage")
              (`self.SetRotation` _output_get)
              (set `PlayerController.CurrentMouseCursor` "Default" (`GameplayStatics.GetPlayerController` 0))
              (set `self.AbleToAttack` true)
              (goto _label :!via `Reset`))))
        (:`NewEnumerator2`
          (`/Engine/EditorBlueprintResources/StandardMacros.DoOnce` false :!label _label_2
            (:`Completed`
              (set `self.AbleToAttack` false)
              (set `self.TargetDistance` _returnvalue)
              (if (not (<= _returnvalue 700.0))
                (`self.Out Range Move` 600.0)
                (`KismetSystemLibrary.Delay` 2.0))
              (`|ExecutionSequence`
                (:`then_0`
                  (`KismetSystemLibrary.Delay` 1.3)
                  (`self.PaladinAbility3` _output_get)
                  (set `self.AbleToAttack` true)
                  (goto _label_2 :!via `Reset`))
                (:`then_1`
                  (`self.SetRotation` _output_get)
                  (`self.PlayAnimMontage` "/Game/FlexibleCombatSystem/NewAnims/Montages/PaladinAbility3.PaladinAbility3")
                  (set `self.SelecetedPoint` false)
                  (set `PlayerController.CurrentMouseCursor` "Default" (`GameplayStatics.GetPlayerController` 0)))))))
        (:`NewEnumerator3`
          (`/Engine/EditorBlueprintResources/StandardMacros.DoOnce` false :!label _label_3
            (:`Completed`
              (if (`self.Initial Overlap`)
                (set `self.TargetDistance` _returnvalue_2)
                (set `self.EnemyFinder` false)
                (if (not (<= _returnvalue_2 3000.0))
                  (`self.Out Range Move` 600.0)
                  (`KismetSystemLibrary.Delay` 2.0))
                (`|ExecutionSequence`
                  (:`then_0`
                    (bind _returnvalue_4 (`GameplayStatics.SpawnEmitterAttached` "/Game/Nodachi_Animset/demo/Particles/P_Sparks.P_Sparks" _mesh (`SkinnedMeshComponent.GetSocketBoneName` _mesh "spine_01") (`SceneComponent.GetSocketLocation` _mesh "spine_01") (struct) (1.0 1.0 1.0) "KeepWorldPosition"))
                    (set `self.AbilityEffect` _returnvalue_4)
                    (`ActorComponent.SetAutoActivate` _radialforce true)
                    (set `RadialForceComponent.bImpulseVelChange` true _radialforce)
                    (`self.SetRotation` _enemylocaiton)
                    (bind (_direction _sweep) (`Timeline|SweepTime` :!via `PlayFromStart`)
                      (:`Update`
                        (bind _sweephitresult (`self.K2_SetActorLocation` (`KismetMathLibrary.VLerp` (`self.K2_GetActorLocation`) _enemylocaiton _sweep) true))
                        (if (`GameplayStatics.BreakHitResult` _sweephitresult)
                          (`self.ApplyForceDamage` 70.0)
                          (`self.CameraShake`)
                          (set `RadialForceComponent.bImpulseVelChange` false (`self.RadialForce`))
                          (`ActorComponent.K2_DestroyComponent` (`self.AbilityEffect`))
                          (set `self.AbleToAttack` true)
                          (goto _label_3 :!via `Reset`)))))
                  (:`then_1`
                    (set `self.SelecetedPoint` false)
                    (set `PlayerController.CurrentMouseCursor` "Default" (`GameplayStatics.GetPlayerController` 0))))))))))))

(event `InputAction|Ability3`
  (params (Key :type "Key Structure"))
  ;[1 1 1] Ability3
  (:`Pressed`
    (`self.StopMovementController`)
    (set `self.SelecetedPoint` true)
    (set `self.AbilityType` "NewEnumerator2")
    (set `PlayerController.CurrentMouseCursor` "Hand" (`GameplayStatics.GetPlayerController` 0))))

(event `InputAction|Hero Ability`
  (params (Key :type "Key Structure"))
  ;[1 1 1] HeroAbility
  (:`Pressed`
    (`self.StopMovementController`)
    (set `self.EnemyFinder` true)
    (set `self.SelecetedPoint` true)
    (set `self.AbilityType` "NewEnumerator3")
    (set `PlayerController.CurrentMouseCursor` "Hand" (`GameplayStatics.GetPlayerController` 0))
    (set `self.AbleToAttack` false)))

(event `InputAction|Ability2`
  (params (Key :type "Key Structure"))
  (bind _mesh (`self.Mesh`))
  ;[1 1 1] Ability2
  (:`Pressed`
    (`self.StopMovementController`)
    (`GameplayStatics.SpawnEmitterAttached` "/Game/Nodachi_Animset/demo/Particles/P_Hit.P_Hit" _mesh (`SkinnedMeshComponent.GetSocketBoneName` _mesh "spine_01") (`SceneComponent.GetSocketLocation` _mesh "spine_01") (struct) (1.0 1.0 1.0) "KeepWorldPosition")
    (if (> (`self.MaxHealth`) 200)
      (set `self.Health` (+ (`self.Health`) 150))
      (else
        (set `self.Health` 200)))))

(fn `ApplyForceDamage`
  (params (BaseDamage :type "Float (single-precision)"))
  (bind _returnvalue (`SceneComponent.GetSocketLocation` (`self.RadialForce`) "None"))
  (bind _outhit (`KismetSystemLibrary.SphereTraceSingleForObjects` :`Start` _returnvalue :`End` _returnvalue :`Radius` 150.0 :`ObjectTypes` (`|MakeArray` "ObjectTypeQuery8" :!type "EObjectTypeQuery Enum") :`DrawDebugType` "ForOneFrame"))
  (bind (_bblockinghit _binitialoverlap _time _distance _location _impactpoint _normal _impactnormal _physmat _hitactor) (`GameplayStatics.BreakHitResult` _outhit))
  (if _bblockinghit
    (`GameplayStatics.ApplyPointDamage` _hitactor BaseDamage _impactpoint _outhit null (cast `/Game/FlexibleCombatSystem/Blueprints/BP_PlayerCharacter` (`GameplayStatics.GetPlayerCharacter` 0) :!pure true))
    (`KismetSystemLibrary.PrintString` "damage")
    (`GameplayStatics.SpawnEmitterAtLocation` "/Game/FlexibleCombatSystem/DemoRoom/VFX/P_FistsImpact.P_FistsImpact" (`self.K2_GetActorLocation` _hitactor))))

(fn `Out Range Move`
  (params (CustomRange :type "Float (double-precision)"))
  (`self.SetRotation` (`self.CachedDestination`))
  (`self.MoveTo` (+ (* (- (`self.TargetDistance`) CustomRange) (`KismetMathLibrary.GetForwardVector` (`self.K2_GetActorRotation`))) (`self.K2_GetActorLocation`))))

(fn `SetRotation`
  (params (To :type "Vector Structure"))
  (bind (_returnvalue_roll _returnvalue_pitch _returnvalue_yaw) (`KismetMathLibrary.BreakRotator` (`KismetMathLibrary.Conv_VectorToRotator` (`KismetMathLibrary.GetDirectionUnitVector` (`self.K2_GetActorLocation`) To))))
  (`self.K2_SetActorRotation` (`KismetMathLibrary.MakeRotator` _returnvalue_roll 0.0 _returnvalue_yaw)))

(fn `UserConstructionScript`
  (`parent.UserConstructionScript`))
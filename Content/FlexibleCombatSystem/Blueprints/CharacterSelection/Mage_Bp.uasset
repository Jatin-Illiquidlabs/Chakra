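; Mage character Blueprint with four click-targeted abilities, including an ultimate.
; Ability inputs stop movement and enter targeting with a hand cursor; Select caches the cursor location and runs the chosen ability, while Cancel exits targeting.
; Abilities cover a triple-projectile call (empty function here), a montage attack that moves closer when out of range, a range-limited teleport with Niagara effect, and a timed ultimate pose.
; DoOnce gates and AbleToAttack guard execution.
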(event `self.ReceiveTick`
  (params (DeltaSeconds :type "Float (single-precision)"))
  (`parent.ReceiveTick` DeltaSeconds))

(event `InputVectorAxis|Mouse2D`
  (params (AxisValue :type "Vector Structure"))
  (if (> (`KismetMathLibrary.Vector_GetAbsMax` AxisValue) 0.0)
    _))

(event `InputAction|CancelAbility`
  (params (Key :type "Key Structure"))
  ;[0.9685 0.9571 1] Abilities
  ;;[1 0 0] Cancel
  (:`Pressed`
    (if (`self.SelecetedPoint`)
      (set `self.SelecetedPoint` false)
      (set `PlayerController.CurrentMouseCursor` "Default" (`GameplayStatics.GetPlayerController` 0))
      (set `self.AbleToAttack` true))))

(event `self.ReceiveBeginPlay`
  (`self.PlayAnimMontage` "/Game/Characters/RevizedAnimations/ShaktiAnims/LevelStart.LevelStart"))

(event `InputAction|Ability1`
  (params (Key :type "Key Structure"))
  ;[0.9685 0.9571 1] Abilities
  (:`Pressed`
    (`self.StopMovementController`)
    (set `self.SelecetedPoint` true)
    (set `self.AbilityType` "NewEnumerator0")
    (set `PlayerController.CurrentMouseCursor` "Hand" (`GameplayStatics.GetPlayerController` 0))))

(event `InputAction|Ability2`
  (params (Key :type "Key Structure"))
  ;[0.9685 0.9571 1] Abilities
  (:`Pressed`
    (`self.StopMovementController`)
    (set `self.SelecetedPoint` true)
    (set `self.AbilityType` "NewEnumerator1")
    (set `PlayerController.CurrentMouseCursor` "Hand" (`GameplayStatics.GetPlayerController` 0))))

(event `InputAction|Ability3`
  (params (Key :type "Key Structure"))
  ;[0.9685 0.9571 1] Abilities
  (:`Pressed`
    (`self.StopMovementController`)
    (set `self.SelecetedPoint` true)
    (set `self.AbilityType` "NewEnumerator2")
    (set `PlayerController.CurrentMouseCursor` "Hand" (`GameplayStatics.GetPlayerController` 0))))

(event `InputAction|Hero Ability`
  (params (Key :type "Key Structure"))
  ;[0.9685 0.9571 1] Abilities
  (:`Pressed`
    (`self.StopMovementController`)
    (set `self.SelecetedPoint` true)
    (set `self.AbilityType` "NewEnumerator3")
    (set `PlayerController.CurrentMouseCursor` "Hand" (`GameplayStatics.GetPlayerController` 0))))

(event `InputAction|Select`
  (params (Key :type "Key Structure"))
  (bind _returnvalue (`KismetMathLibrary.Vector_Distance` (`self.CachedDestination`) (`self.K2_GetActorLocation`)))
  (bind _returnvalue_2 (`KismetMathLibrary.Vector_Distance` (`self.CachedDestination`) (`self.K2_GetActorLocation`)))
  (bind _returnvalue_3 (`KismetMathLibrary.Vector_Distance` (`self.CachedDestination`) (`self.K2_GetActorLocation`)))
  ;[0.9685 0.9571 1] Abilities
  (:`Pressed`
    (if (`self.SelecetedPoint`)
      (bind _output_get (set `self.CachedDestination` (`.Location` (`self.GetLocationUnderCursor`))))
      (switch `/Game/FlexibleCombatSystem/Blueprints/PaladinChar_AbilityType` (`self.AbilityType`)
        (:`NewEnumerator0`
          (`/Engine/EditorBlueprintResources/StandardMacros.DoOnce` false :!label _label
            (:`Completed`
              (set `self.AbleToAttack` false)
              (`self.PlayAnimMontage` "/Game/Characters/RevizedAnimations/ShaktiAnims/Shakti_AbilityOneMontage.Shakti_AbilityOneMontage")
              (`self.SetRotation` _output_get)
              (set `PlayerController.CurrentMouseCursor` "Default" (`GameplayStatics.GetPlayerController` 0))
              (set `self.SelecetedPoint` false)
              (`KismetSystemLibrary.Delay` 0.4)
              (`self.SpawnTripleProjetile` _output_get _output_get _output_get)
              (set `self.AbleToAttack` true)
              (goto _label :!via `Reset`))))
        (:`NewEnumerator1`
          (`/Engine/EditorBlueprintResources/StandardMacros.DoOnce` false :!label _label_2
            (:`Completed`
              (set `self.AbleToAttack` false)
              (set `self.TargetDistance` _returnvalue_3)
              (if (<= _returnvalue_3 1200.0)
                (`self.PlayAnimMontage` "/Game/FlexibleCombatSystem/NewAnims/Montages/attack_01_Montage1.attack_01_Montage1")
                (else
                  (`self.Out Range Move` 600.0)
                  (`KismetSystemLibrary.Delay` 2.0)))
              (`self.SetRotation` _output_get)
              (set `PlayerController.CurrentMouseCursor` "Default" (`GameplayStatics.GetPlayerController` 0))
              (set `self.SelecetedPoint` false)
              (set `self.AbleToAttack` true)
              (goto _label_2 :!via `Reset`))))
        (:`NewEnumerator2`
          (`/Engine/EditorBlueprintResources/StandardMacros.DoOnce` false :!label _label_3
            (:`Completed`
              (set `self.TargetDistance` _returnvalue_2)
              (set `self.AbleToAttack` false)
              (if (<= _returnvalue_2 700.0)
                (`self.K2_TeleportTo` _output_get)
                (`NiagaraFunctionLibrary.SpawnSystemAtLocation` "/Game/Plugins/DarkSocerer_Animset/demo/FX/NS_FireToon.NS_FireToon" _output_get)
                (`self.SetRotation` _output_get)
                (set `self.SelecetedPoint` false)
                (set `PlayerController.CurrentMouseCursor` "Default" (`GameplayStatics.GetPlayerController` 0))
                (set `self.AbleToAttack` true)
                (goto _label_3 :!via `Reset`)
                (else
                  (goto _label_3 :!via `Reset`))))))
        (:`NewEnumerator3`
          (`/Engine/EditorBlueprintResources/StandardMacros.DoOnce` false :!label _label_4
            (:`Completed`
              (set `self.TargetDistance` _returnvalue)
              (if (<= _returnvalue 700.0)
                (set `self.UltiActivated_0` true)
                (set `self.AbleToAttack` false)
                (bind _returnvalue_4 (`self.PlayAnimMontage` "/Game/FlexibleCombatSystem/NewAnims/Montages/UltiStartü_Montage.UltiStartü_Montage"))
                (`KismetSystemLibrary.Delay` _returnvalue_4)
                (set `self.UltiPose` true)
                (`KismetSystemLibrary.Delay` 3.0)
                (set `self.UltiPose` false)
                (set `self.UltiActivated_0` false)
                (bind _returnvalue_5 (`self.PlayAnimMontage` "/Game/FlexibleCombatSystem/NewAnims/Montages/UltiEndPose_Montage.UltiEndPose_Montage"))
                (`KismetSystemLibrary.Delay` _returnvalue_5)
                (set `self.SelecetedPoint` false)
                (set `PlayerController.CurrentMouseCursor` "Default" (`GameplayStatics.GetPlayerController` 0))
                (set `self.AbleToAttack` true)
                (goto _label_4 :!via `Reset`)))))))))

(fn `Out Range Move`
  (params (CustomRange :type "Float (double-precision)"))
  (`self.SetRotation` (`self.CachedDestination`))
  (`self.MoveTo` (+ (* (- (`self.TargetDistance`) CustomRange) (`KismetMathLibrary.GetForwardVector` (`self.K2_GetActorRotation`))) (`self.K2_GetActorLocation`))))

(fn `SetRotation`
  (params (To :type "Vector Structure"))
  (bind (_returnvalue_roll _returnvalue_pitch _returnvalue_yaw) (`KismetMathLibrary.BreakRotator` (`KismetMathLibrary.Conv_VectorToRotator` (`KismetMathLibrary.GetDirectionUnitVector` (`self.K2_GetActorLocation`) To))))
  (`self.K2_SetActorRotation` (`KismetMathLibrary.MakeRotator` _returnvalue_roll 0.0 _returnvalue_yaw)))

(fn `SpawnPorjectileAbility`
  (params (InSocketName :type Name) (Class :type "Actor Class Reference") (Target :type "SceneComponent Object Reference") (`Spawn Transform Rotation` :type "Rotator Structure"))
  (bind _returnvalue (`SceneComponent.GetSocketLocation` Target InSocketName))
  (bind _mesh (`self.Mesh`))
  (`|ExecutionSequence`
    (:`then_0`
      (`GameplayStatics.SpawnEmitterAtLocation` "/Game/DarkSocerer_Animset/demo/FX/P_Hit.P_Hit" _returnvalue))
    (:`then_1`
      (bind _returnvalue_2 (`|SpawnActorFromClass` Class (`KismetMathLibrary.MakeTransform` _returnvalue `Spawn Transform Rotation`) "Undefined" "OverrideRootScale" null null))
      (set `self.SpawnProjectile` _returnvalue_2)
      (`GameplayStatics.SpawnEmitterAttached` null _mesh (`SkinnedMeshComponent.GetSocketBoneName` _mesh "hand_r") (0.0 0.0 0.0) (struct) (0.3 0.3 0.3))
      (`self.CameraShake`))))

(fn `SpawnTripleProjetile`
  (params (A :type "Vector Structure") (A2 :type "Vector Structure") (A3 :type "Vector Structure")))

(fn `TraceArrow`
  (params (Target :type "SceneComponent Object Reference") (End :type "Vector Structure"))
  (`KismetSystemLibrary.LineTraceMultiForObjects` :`Start` (`SceneComponent.GetSocketLocation` Target "None") :`End` End :`ObjectTypes` (`|MakeArray` "ObjectTypeQuery1" :!type "EObjectTypeQuery Enum") :`DrawDebugType` "ForOneFrame"))

(fn `UserConstructionScript`
  (`parent.UserConstructionScript`))
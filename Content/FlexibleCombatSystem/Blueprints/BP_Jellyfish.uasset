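; BP_Jellyfish is an actor that moves its jellyfish component back and forth along a spline.
; BeginPlay sets the timeline play rate from TimelineLength, then starts movement in the direction given by IsMovingForward.
; Timeline updates lerp distance to the last spline point and set world location; finishing flips direction and restarts.
; Tangent-based rotation logic is present but unconnected, so only position changes.
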(event `self.ReceiveBeginPlay`
  (`TimelineComponent.SetPlayRate` (`self.JellyfishMovement_Timeline`) (`self.TimelineLength`))
  (`self.StartMovement` (`self.IsMovingForward`)))

(event `StartMovement`
  (params (IsMovingForward :type Boolean))
  (bind _spline (`self.Spline`))
  (if IsMovingForward
    (bind (_direction _distance) (`Timeline|JellyfishMovement_Timeline` :!via `PlayFromStart` :!label _label)
      (:`Update`
        (`SceneComponent.K2_SetWorldLocation` (`self.S_Jellyfish`) (`SplineComponent.GetLocationAtDistanceAlongSpline` (`self.Spline`) (`KismetMathLibrary.Lerp` 0.0 (`SplineComponent.GetDistanceAlongSplineAtSplinePoint` _spline (- (`SplineComponent.GetNumberOfSplinePoints` _spline) 1)) _distance) "World") false false))
      (:`Finished`
        (bind _output_get (set `self.IsMovingForward` (not (`self.IsMovingForward`))))
        (set `self.SplineIndex` (* (`self.SplineIndex`) -1))
        (`self.StartMovement` _output_get)))
    (else
      (goto _label :!via `ReverseFromEnd`))))

(fn `UserConstructionScript`)
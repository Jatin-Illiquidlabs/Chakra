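; Base projectile actor for the combat system that applies point damage when its sphere component hits something.
; An incoming event stores the attack damage, and each hit applies it with the player character as damage causer and spawns an impact emitter.
; The hit also starts the Move timeline, which lerps the sphere from the actor's location toward the player's through MoveComponentTo.
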(event `self.ReceiveTick`
  (params (DeltaSeconds :type "Float (single-precision)")))

(event `/Game/FlexibleCombatSystem/Blueprints/Interfaces/I_WeaponInterface.SendAttackDamageToWeapon`
  (params (AttackDamage :type Integer))
  (set `self.WeaponOutputDamage` (`KismetMathLibrary.Conv_IntToDouble` AttackDamage)))

(event `self.Sphere.OnComponentHit`
  (params (HitComponent :type "PrimitiveComponent Object Reference") (OtherActor :type "Actor Object Reference") (OtherComp :type "PrimitiveComponent Object Reference") (NormalImpulse :type "Vector Structure") (Hit :type "HitResult Structure (by ref)"))
  (bind (_bblockinghit _binitialoverlap _time _distance _location _impactpoint _normal _impactnormal _physmat _hitactor) (`GameplayStatics.BreakHitResult` Hit))
  (`GameplayStatics.ApplyPointDamage` _hitactor (`self.WeaponOutputDamage`) _impactpoint Hit null (cast `/Game/FlexibleCombatSystem/Blueprints/BP_PlayerCharacter` (`GameplayStatics.GetPlayerCharacter` 0) :!pure true))
  (`GameplayStatics.SpawnEmitterAtLocation` "/Game/AdvancedMagicFX12/particles/P_ky_hit_dark.P_ky_hit_dark" _impactpoint)
  (bind (_direction _time_2) (`Timeline|Move` :!via `PlayFromStart`)
    (:`Update`
      (`KismetSystemLibrary.MoveComponentTo` (`self.Sphere`) (`KismetMathLibrary.VLerp` (`self.K2_GetActorLocation`) (`self.K2_GetActorLocation` (cast `/Game/FlexibleCombatSystem/Blueprints/BP_PlayerCharacter` (`GameplayStatics.GetPlayerCharacter` 0) :!pure true)) _time_2)))))

(fn `UserConstructionScript`)
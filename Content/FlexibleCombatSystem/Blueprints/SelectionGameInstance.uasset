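; Game instance that wraps PlayFab backend calls for login, title and user data, player statistics and leaderboards.
; Custom-ID login creates accounts as needed, then sets the display name from the player's nickname.
; Events call Client or Admin APIs directly or run CloudScript functions with JSON parameters.
; Results are mostly just printed on screen, with leaderboard rows also stored, and most failures route to a shared Failed function that prints the error.
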(event `GetNumberOfEnemiesPerWaveSucces`
  (params (result :type "AdminGetTitleDataResult Structure") (customData :type "Object Object Reference"))
  (`KismetSystemLibrary.PrintString` (`PlayFabJsonObject.GetStringField` (`.Data` (break `AdminGetTitleDataResult` result)) (`self.NumberOfEnemiesKey`)) true true (struct :`R` 0.206457 :`G` 1.0 :`A` 1.0)))

(event `GetNumberOfEnemiesFromPlayFab`
  (`PlayFabAdminAPI.GetTitleData` (make `AdminGetTitleDataRequest` (`self.NumberOfEnemiesKey`)) (delegate `GetNumberOfEnemiesPerWaveSucces`) (delegate `FailedNumber`)))

(event `FailedNumber`
  (params (error :type "PlayFabError Structure") (customData :type "Object Object Reference"))
  (`self.Failed` error))

(event `CustomEvent`
  (params (error :type "PlayFabError Structure") (customData :type "Object Object Reference"))
  (`KismetSystemLibrary.PrintString` "Error"))

(event `FailedConnect`
  (params (error :type "PlayFabError Structure") (customData :type "Object Object Reference"))
  (`self.Failed` error))

(event `UpdateDisplaySucces`
  (params (result :type "ClientUpdateUserTitleDisplayNameResult Structure") (customData :type "Object Object Reference"))
  (`KismetSystemLibrary.PrintString` (stale `SuccesConnect` _returnvalue) true true (struct :`R` 1.0 :`G` 1.0 :`B` 1.0 :`A` 1.0) 15.0))

(event `SuccesConnect`
  (params (result :type "ClientLoginResult Structure") (customData :type "Object Object Reference"))
  (bind _returnvalue (`EIK_BlueprintFunctions.GetPlayerNickname` 0))
  (`PlayFabClientAPI.UpdateUserTitleDisplayName` (make `ClientUpdateUserTitleDisplayNameRequest` null _returnvalue) (delegate `UpdateDisplaySucces`) (delegate `UpdateDisplayFailed`)))

(event `ConnectToPlayFab`
  (params (`Custom Id` :type String))
  (`PlayFabClientAPI.LoginWithCustomID` (make `ClientLoginWithCustomIDRequest` true `Custom Id`) (delegate `SuccesConnect`) (delegate `FailedConnect`)))

(event `UpdateDisplayFailed`
  (params (error :type "PlayFabError Structure") (customData :type "Object Object Reference"))
  (`self.Failed` error))

(event `ChangePlayerName`
  (params (`Play Fab Id` :type String)))

(event `OnSucces`
  (params (result :type "ClientExecuteCloudScriptResult Structure") (customData :type "Object Object Reference"))
  (`KismetSystemLibrary.PrintString` "Executre Succes"))

(event `UpdateStats`
  (params (StringValue :type String))
  (bind _json (`self.JSON`))
  (set `self.JSON` (`PlayFabJsonObject.ConstructJsonObject`))
  (`PlayFabJsonObject.SetStringField` _json "testdata" "")
  (`PlayFabClientAPI.ExecuteCloudScript` (make `ClientExecuteCloudScriptRequest` null "testUpdate" _json) (delegate `OnSucces`) (delegate `FailedExecuted`)))

(event `FailedExecuted`
  (params (error :type "PlayFabError Structure") (customData :type "Object Object Reference"))
  (`self.Failed` error))

(event `SuccesGetTitleData`
  (params (result :type "ClientGetTitleDataResult Structure") (customData :type "Object Object Reference"))
  (`KismetSystemLibrary.PrintString` (`PlayFabJsonObject.GetStringField` (`.Data` (break `ClientGetTitleDataResult` result)) (stale `GetTitleData` `Key Name`))))

(event `GetTitleData`
  (params (`Key Name` :type String))
  (set `self.JSON` (`PlayFabJsonObject.ConstructJsonObject`))
  (`PlayFabJsonObject.SetStringField` (`self.JSON`) `Key Name` "Turn Timer")
  (`PlayFabClientAPI.GetTitleData` (make `ClientGetTitleDataRequest` `Key Name`) (delegate `SuccesGetTitleData`) (delegate `FieldGetTitleData`)))

(event `FieldGetTitleData`
  (params (error :type "PlayFabError Structure") (customData :type "Object Object Reference"))
  (`self.Failed` error))

(event `SuccesGetTitleSctript`
  (params (result :type "ClientExecuteCloudScriptResult Structure") (customData :type "Object Object Reference"))
  (`KismetSystemLibrary.PrintString` (`PlayFabJsonValue.AsString` (`PlayFabJsonObject.GetField` (`.FunctionResult` (break `ClientExecuteCloudScriptResult` result)) "Value"))))

(event `GetTitleDataScript`
  (params (`Key Name` :type String))
  (bind _json (`self.JSON`))
  (set `self.JSON` (`PlayFabJsonObject.ConstructJsonObject`))
  (`PlayFabJsonObject.SetStringField` _json `Key Name` "Turn Timer")
  (`PlayFabClientAPI.ExecuteCloudScript` (make `ClientExecuteCloudScriptRequest` null "GetTitleData" _json true) (delegate `SuccesGetTitleSctript`) (delegate `FailedTitleScript`)))

(event `FailedTitleScript`
  (params (error :type "PlayFabError Structure") (customData :type "Object Object Reference"))
  (`self.Failed` error))

(event `Get User Data1 Succes`
  (params (result :type "AdminGetUserDataResult Structure") (customData :type "Object Object Reference"))
  (bind _data (break `AdminGetUserDataResult` result))
  (bind _returnvalue (`PlayFabJsonValue.AsObject` (`PlayFabJsonObject.GetField` _data (`|GetArrayItem` (`PlayFabJsonObject.GetFieldNames` _data)))))
  (`KismetSystemLibrary.PrintString` (`PlayFabJsonObject.GetStringField` _returnvalue (`|GetArrayItem` (`PlayFabJsonObject.GetFieldNames` _returnvalue)))))

(event `GetUserData1`
  (params (Key :type String))
  (`PlayFabAdminAPI.GetUserData` (make `AdminGetUserDataRequest` 0 Key) (delegate `Get User Data1 Succes`) (delegate `GetUserData1Failed`)))

(event `GetUserData1Failed`
  (params (error :type "PlayFabError Structure") (customData :type "Object Object Reference"))
  (`self.Failed` error))

(event `GetUserData2Succes`
  (params (result :type "ClientExecuteCloudScriptResult Structure") (customData :type "Object Object Reference"))
  (`KismetSystemLibrary.PrintString` (`PlayFabJsonValue.AsString` (`PlayFabJsonObject.GetField` (`.FunctionResult` (break `ClientExecuteCloudScriptResult` result)) "Value"))))

(event `GetUserData2`
  (params (KeyName :type String))
  (bind _json (`self.JSON`))
  (set `self.JSON` (`PlayFabJsonObject.ConstructJsonObject`))
  (`PlayFabJsonObject.SetStringField` _json KeyName "Wins")
  (`PlayFabClientAPI.ExecuteCloudScript` (make `ClientExecuteCloudScriptRequest` null "testTitleData" _json true) (delegate `GetUserData2Succes`) (delegate `GetUserData2Failed`)))

(event `GetUserData2Failed`
  (params (error :type "PlayFabError Structure") (customData :type "Object Object Reference"))
  (`self.Failed` error))

(event `SuccesLeaderBoards`
  (params (result :type "ClientGetLeaderboardResult Structure") (customData :type "Object Object Reference"))
  (for _array_element (`.Leaderboard` (break `ClientGetLeaderboardResult` result))
    (`KismetSystemLibrary.PrintString` (`PlayFabJsonValue.AsString` (`PlayFabJsonObject.GetField` _array_element "pscore")))))

(event `LeaderBoard`
  (`PlayFabClientAPI.GetLeaderboard` (make `ClientGetLeaderboardRequest` null 10 null 0 "Test Wins") (delegate `SuccesLeaderBoards`) (delegate `FailedLeaderBoard`)))

(event `FailedLeaderBoard`
  (params (error :type "PlayFabError Structure") (customData :type "Object Object Reference"))
  (`self.Failed` error))

(event `UpdateScoreSucces`
  (params (result :type "ClientExecuteCloudScriptResult Structure") (customData :type "Object Object Reference"))
  (`KismetSystemLibrary.PrintString` "ScoreSucces"))

(event `UpdateScore`
  (params (StringValue :type String))
  (bind _json (`self.JSON`))
  (set `self.JSON` (`PlayFabJsonObject.ConstructJsonObject`))
  (`PlayFabJsonObject.SetField` _json "pscore" (`PlayFabJsonValue.ConstructJsonValueString` StringValue))
  (`PlayFabClientAPI.ExecuteCloudScript` (make `ClientExecuteCloudScriptRequest` null "UpdatePlayerData" _json true) (delegate `UpdateScoreSucces`) (delegate `UpdateScoreFiled`)))

(event `UpdateScoreFiled`
  (params (error :type "PlayFabError Structure") (customData :type "Object Object Reference")))

(event `SendScoreSucces`
  (params (result :type "ClientUpdatePlayerStatisticsResult Structure") (customData :type "Object Object Reference"))
  (`KismetSystemLibrary.PrintString` "KillsSended" true true (struct :`R` 1.0 :`G` 0.976174 :`A` 1.0) 5.0))

(event `SendScoreAsStatic`
  (params (Score :type Integer))
  (bind _output_get (set `self.JSON` (`PlayFabJsonObject.ConstructJsonObject`)))
  (`PlayFabJsonObject.SetStringField` _output_get "StatisticName" (`self.ScoreStats`))
  (`PlayFabJsonObject.SetNumberField` _output_get "Value" (`KismetMathLibrary.Conv_IntToDouble` Score))
  (`PlayFabClientAPI.UpdatePlayerStatistics` (make `ClientUpdatePlayerStatisticsRequest` null (`|MakeArray` (`self.JSON`))) (delegate `SendScoreSucces`) (delegate `SendScoreFailed`)))

(event `SendScoreFailed`
  (params (error :type "PlayFabError Structure") (customData :type "Object Object Reference"))
  (`self.Failed` error))

(event `GetLeaderBoardSucces`
  (params (result :type "ClientGetLeaderboardResult Structure") (customData :type "Object Object Reference"))
  (bind _leaderboard (break `ClientGetLeaderboardResult` result))
  (set `self.Leaderboard_0` _leaderboard)
  (`KismetSystemLibrary.PrintString` (`KismetStringLibrary.Concat_StrStr` "POSITION" " | " "USERNAME" " |" "SCORE"))
  (for _array_element _leaderboard
    (set `self.ArrayLeaderBoaard` _array_element)
    (bind _returnvalue (`PlayFabJsonObject.GetStringField` _array_element "DisplayName"))
    (set `self.PlayerNames` (`|MakeArray` _returnvalue))
    (bind _output_get (set `self.LeaderBoardStats` (`KismetStringLibrary.Concat_StrStr` (`PlayFabJsonObject.GetStringField` _array_element "Position") " " _returnvalue " " (`PlayFabJsonObject.GetStringField` _array_element "StatValue"))))
    (`KismetSystemLibrary.PrintText` (`KismetTextLibrary.Conv_StringToText` _output_get) true true (struct :`R` 1.0 :`G` 0.816154 :`A` 1.0) 20.0))
  (`KismetSystemLibrary.PrintString` "EndScore"))

(event `GetLeaderBoard`
  (`PlayFabClientAPI.GetLeaderboard` (make `ClientGetLeaderboardRequest` null 10 null 0 "ScoreStats") (delegate `GetLeaderBoardSucces`) (delegate `GetLeaderBoardFailed`)))

(event `GetLeaderBoardFailed`
  (params (error :type "PlayFabError Structure") (customData :type "Object Object Reference"))
  (`self.Failed` error))

(fn `Failed`
  (params (Errors :type "PlayFabError Structure"))
  (bind (_haserror _errorcode _errorname _errormessage _errordetails) (break `PlayFabError` Errors))
  (`KismetSystemLibrary.PrintString` _errorname true true (struct :`G` 0.66 :`B` 1.0 :`A` 1.0) 5.0)
  (`KismetSystemLibrary.PrintString` _errormessage true true (struct :`G` 0.66 :`B` 1.0 :`A` 1.0) 5.0)
  (`KismetSystemLibrary.PrintString` _errordetails true true (struct :`G` 0.66 :`B` 1.0 :`A` 1.0) 5.0))
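; Playable paladin-style hero character with four cooldown-gated abilities: sword teleport, self-heal, targeted spawn and enemy-seeking ultimate.
; Targeted abilities set a cursor selection state; Select then walks into range if needed, turns and plays a montage.
; The ultimate finds enemies by sphere trace under the cursor, timeline-lerps toward them and deals radial-force impact damage on capsule hits.
; Tick also maps total level to the level component, while talent functions adjust stats, some still empty.
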(event `self.ReceiveBeginPlay`
  (`parent.ReceiveBeginPlay`))

(event `self.ReceiveTick`
  (params (DeltaSeconds :type "Float (single-precision)"))
  (bind (_hit _location) (`self.GetLocationUnderCursor`))
  (`parent.ReceiveTick` DeltaSeconds)
  (`|ExecutionSequence`
    (:`then_0`
      (`RadialForceComponent.FireImpulse` (`self.RadialForce`))
      (set `self.Initial Overlap_0` (`self.Initial Overlap_0`))
      (bind _output_get (set `self.EnemyFinder` (`self.EnemyFinder`)))
      (if _output_get
        (set `self.CachedDestination` _location)
        (bind _outhit (`KismetSystemLibrary.SphereTraceSingleForObjects` :`Start` _location :`End` _location :`Radius` 50.0 :`ObjectTypes` (`|MakeArray` "ObjectTypeQuery8" :!type "EObjectTypeQuery Enum") :`TraceColor` (struct :`R` 0.155884 :`B` 1.0 :`A` 1.0) :`TraceHitColor` (struct :`G` 1.0 :`B` 0.95483 :`A` 1.0)))
        (bind (_bblockinghit _binitialoverlap _time _distance _location_2 _impactpoint _normal _impactnormal _physmat _hitactor) (`GameplayStatics.BreakHitResult` _outhit))
        (bind _output_get_2 (set `self.Initial Overlap_1` _binitialoverlap))
        (if _output_get_2
          (set `self.EnemyLocaiton` (`self.K2_GetActorLocation` (cast `/Game/FlexibleCombatSystem/Blueprints/AI/BP_EnemyAI` _hitactor :!pure true))))))
    (:`then_1`
      (`self.UpgradeLevel`))))

(event `InputAction|CancelAbility`
  (params (Key :type "Key Structure"))
  ;[1 0 0] Cancel
  (:`Pressed`
    (if (and (`self.SelecetedPoint`) (not (`self.IsAttacking`)))
      (set `self.SelecetedPoint` false)
      (set `PlayerController.CurrentMouseCursor` "Default" (`GameplayStatics.GetPlayerController` 0))
      (set `self.AbleToAttack` true)
      (set `self.EnemyFinder` false)
      (set `self.AbilityType` "NewEnumerator4"))))

(event `InputAction|Ability1`
  (params (Key :type "Key Structure"))
  ;[1 1 1] Ability1
  (:`Pressed`
    (if (`self.CanAttack_0`)
      (`self.Ability1`))))

(event `Ability1`
  ;[1 1 1] Ability1
  (if (`self.HasTeleportPoint`)
    (bind _returnvalue (`GameplayStatics.GetActorOfClass` "/Game/FlexibleCombatSystem/Blueprints/Weapons/PaladinAbility/BP_TeleportSword.BP_TeleportSword_C"))
    (if (`/Game/FlexibleCombatSystem/Blueprints/Weapons/PaladinAbility/BP_TeleportSword.Floor` _returnvalue)
      (if (`/Game/FlexibleCombatSystem/Blueprints/Weapons/PaladinAbility/BP_TeleportSword.Located` _returnvalue)
        (bind (_returnvalue_x _returnvalue_y) (`KismetMathLibrary.BreakVector` (`self.K2_GetActorLocation` _returnvalue)))
        (`self.K2_TeleportTo` (`KismetMathLibrary.MakeVector` _returnvalue_x _returnvalue_y 90.0))
        (`NiagaraFunctionLibrary.SpawnSystemAtLocation` "/Game/Plugins/DarkSocerer_Animset/demo/FX/NS_FireToon.NS_FireToon" (`KismetMathLibrary.MakeVector` _returnvalue_x _returnvalue_y 50.0))
        (set `self.SelecetedPoint` false)
        (set `self.AbleToAttack` true)
        (set `self.AbilityType` "NewEnumerator4")
        (if (`self.Gain25Armor`)
          (if (and (<= (`self.Health`) 175) (> (`self.MaxHealth`) 200))
            (set `self.Health` (+ (`self.Health`) 25))
            (else
              (set `self.Health` 200)))
          (else
            (`self.K2_DestroyActor` _returnvalue)
            (set `self.AbilityType` "NewEnumerator4")
            (set `self.HasTeleportPoint` false)
            (`self.ExitAttack` true)))))
    (else
      (`self.ExitAttack` false)
      (set `self.SelecetedPoint` true)
      (set `self.AbilityType` "NewEnumerator0")
      (set `PlayerController.CurrentMouseCursor` "Hand" (`GameplayStatics.GetPlayerController` 0)))))

(event `InputAction|Select`
  (params (Key :type "Key Structure"))
  (bind _enemylocaiton (`self.EnemyLocaiton`))
  (bind _radialforce (`self.RadialForce`))
  (bind _returnvalue (`KismetMathLibrary.Vector_Distance` (`self.CachedDestination`) (`self.K2_GetActorLocation`)))
  (bind _returnvalue_2 (`KismetMathLibrary.Vector_Distance` (`self.CachedDestination`) (`self.K2_GetActorLocation`)))
  (bind _returnvalue_3 (`KismetMathLibrary.Vector_Distance` (`self.CachedDestination`) (`self.K2_GetActorLocation`)))
  ;[0.8785 1 0] Selection
  (:`Pressed`
    (if (`self.SelecetedPoint`)
      (bind _output_get (set `self.CachedDestination` (`.Location` (`self.GetLocationUnderCursor`))))
      (switch `/Game/FlexibleCombatSystem/Blueprints/PaladinChar_AbilityType` (`self.AbilityType`)
        (:`NewEnumerator0`
          (if (>= (`self.Ability1C`) 1.0)
            (`/Engine/EditorBlueprintResources/StandardMacros.DoOnce` false :!label _label
              (:`Completed`
                (if (`self.IsAttacking`)
                  (goto _label :!via `Reset`)
                  (else
                    (set `self.IsAttacking` true)
                    (set `self.AbleToAttack` false)
                    (set `self.TargetDistance` _returnvalue_3)
                    (if (not (<= _returnvalue_3 1200.0))
                      (`self.Out Range Move` 600.0)
                      (`KismetSystemLibrary.Delay` 2.0))
                    (bind _output_get_2 (set `self.Current Anim Montage` "/Game/Characters/RevizedAnimations/DevaAnims/Deva_AbilityOneMontage.Deva_AbilityOneMontage"))
                    (`self.PlayAnimMontage` _output_get_2)
                    (set `self.Ability1C` 0.0)
                    (`self.SetRotation` _output_get))))))
          (set `self.AbilityType` "NewEnumerator4")
          (set `PlayerController.CurrentMouseCursor` "Default" (`GameplayStatics.GetPlayerController` 0))
          (set `self.AbleToAttack` true)
          (goto _label :!via `Reset`))
        (:`NewEnumerator2`
          (`/Engine/EditorBlueprintResources/StandardMacros.DoOnce` false :!label _label_2
            (:`Completed`
              (if (`self.IsAttacking`)
                (goto _label_2 :!via `Reset`)
                (else
                  (set `self.IsAttacking` true)
                  (set `self.AbleToAttack` false)
                  (set `self.TargetDistance` _returnvalue)
                  (if (not (<= _returnvalue 700.0))
                    (`self.Out Range Move` 600.0)
                    (`KismetSystemLibrary.Delay` 2.0))
                  (`|ExecutionSequence`
                    (:`then_0`
                      (`KismetSystemLibrary.Delay` 1.3)
                      (`self.PaladinAbility3` _output_get)
                      (set `self.AbleToAttack` true)
                      (goto _label_2 :!via `Reset`))
                    (:`then_1`
                      (`self.SetRotation` _output_get)
                      (bind _output_get_3 (set `self.Current Anim Montage` "/Game/Characters/RevizedAnimations/DevaAnims/Deva_AbilityThreeMontage.Deva_AbilityThreeMontage"))
                      (`self.PlayAnimMontage` _output_get_3)
                      (set `self.SelecetedPoint` false)
                      (set `PlayerController.CurrentMouseCursor` "Default" (`GameplayStatics.GetPlayerController` 0))
                      (set `self.AbilityType` "NewEnumerator4"))))))))
        (:`NewEnumerator3`
          (`/Engine/EditorBlueprintResources/StandardMacros.DoOnce` false :!label _label_3
            (:`Completed`
              (if (`self.IsAttacking`)
                (goto _label_3 :!via `Reset`)
                (else
                  (set `self.IsAttacking` true)
                  (if (`self.Initial Overlap_1`)
                    (set `self.TargetDistance` _returnvalue_2)
                    (set `self.EnemyFinder` false)
                    (if (not (<= _returnvalue_2 3000.0))
                      (`self.Out Range Move` 600.0)
                      (`KismetSystemLibrary.Delay` 2.0))
                    (`|ExecutionSequence`
                      (:`then_0`
                        (set `self.UltiActivated` true)
                        (bind _output_get_4 (set `self.Current Anim Montage` "/Game/FlexibleCombatSystem/NewAnims/Montages/Anim_combo_03_3_Montage.Anim_combo_03_3_Montage"))
                        (`self.PlayAnimMontage` _output_get_4)
                        (`ActorComponent.SetAutoActivate` _radialforce true)
                        (set `RadialForceComponent.bImpulseVelChange` true _radialforce)
                        (`self.SetRotation` _enemylocaiton)
                        (bind (_direction _sweep) (`Timeline|SweepTime` :!via `PlayFromStart`)
                          (:`Update`
                            (`self.K2_SetActorLocation` (`KismetMathLibrary.VLerp` (`self.K2_GetActorLocation`) _enemylocaiton _sweep) true)
                            (set `RadialForceComponent.bImpulseVelChange` false (`self.RadialForce`))
                            (set `self.AbleToAttack` true)
                            (goto _label_3 :!via `Reset`))))
                      (:`then_1`
                        _)))
                  (set `self.EnemyFinder` false)
                  (set `self.SelecetedPoint` false)
                  (set `PlayerController.CurrentMouseCursor` "Default" (`GameplayStatics.GetPlayerController` 0))
                  (set `self.AbleToAttack` true)
                  (set `RadialForceComponent.bImpulseVelChange` false (`self.RadialForce`))
                  (set `self.UltiActivated` true)
                  (set `self.IsAttacking` false)
                  (set `self.AbilityType` "NewEnumerator4")
                  (goto _label_3 :!via `Reset`))))))))))

(event `InputAction|Ability3`
  (params (Key :type "Key Structure"))
  ;[1 1 1] Ability3
  (:`Pressed`
    (`self.Ability3`)))

(event `Ability3`
  ;[1 1 1] Ability3
  (if (and (`self.CanAttack_0`) (>= (`self.Ability3C`) 1.0))
    (`self.ExitAttack` false)
    (set `self.SelecetedPoint` true)
    (set `self.AbilityType` "NewEnumerator2")
    (set `PlayerController.CurrentMouseCursor` "Hand" (`GameplayStatics.GetPlayerController` 0))
    (set `self.Ability3C` 0.0)))

(event `InputAction|Hero Ability`
  (params (Key :type "Key Structure"))
  ;[1 1 1] HeroAbility
  (:`Pressed`
    (`self.Ultimate`)))

(event `Ultimate`
  ;[1 1 1] HeroAbility
  (if (and (`self.CanAttack_0`) (>= (`self.UltiC`) 1.0))
    (`self.ExitAttack` false)
    (set `self.EnemyFinder` true)
    (set `self.SelecetedPoint` true)
    (set `self.AbilityType` "NewEnumerator3")
    (set `PlayerController.CurrentMouseCursor` "Hand" (`GameplayStatics.GetPlayerController` 0))
    (set `self.AbleToAttack` false)
    (set `self.UltiC` 0.0)))

(event `Ability2`
  (bind _mesh (`self.Mesh`))
  ;[1 1 1] Ability2
  (if (and (`self.CanAttack_0`) (>= (`self.Ability2C`) 1.0))
    (`self.ExitAttack` false)
    (`NiagaraFunctionLibrary.SpawnSystemAttached` "/Game/FlexibleCombatSystem/SelectedVFX/new_selected/Deva/P_Implosion_03_Selected.P_Implosion_03_Selected" _mesh (`SkinnedMeshComponent.GetSocketBoneName` _mesh "spine_01") (`SceneComponent.GetSocketLocation` _mesh "spine_01") (struct) "KeepWorldPosition")
    (set `self.Ability2C` 0.0)
    (if (> (`self.MaxHealth`) 200)
      (set `self.Health` (+ (`self.Health`) 150))
      (else
        (set `self.Health` 200)))))

(event `InputAction|Ability2`
  (params (Key :type "Key Structure"))
  ;[1 1 1] Ability2
  (:`Pressed`
    (`self.Ability2`)))

(event `self.CapsuleComponent.OnComponentHit`
  (params (HitComponent :type "PrimitiveComponent Object Reference") (OtherActor :type "Actor Object Reference") (OtherComp :type "PrimitiveComponent Object Reference") (NormalImpulse :type "Vector Structure") (Hit :type "HitResult Structure (by ref)"))
  (bind (_bblockinghit _binitialoverlap _time _distance _location) (`GameplayStatics.BreakHitResult` Hit))
  ;[0.8785 1 0] Selection
  (if (!= OtherActor (cast `/Game/FlexibleCombatSystem/Blueprints/BP_PlayerCharacter` (`GameplayStatics.GetPlayerCharacter` 0) :!pure true))
    (bind _output_get (set `self.Blocking Hit` _bblockinghit))
    (if (and (`self.UltiActivated`) _output_get)
      (`self.ApplyForceDamage` 0.0 Hit OtherActor _location)
      (`/Engine/EditorBlueprintResources/StandardMacros.DoOnce` false :!label _label_4
        (:`Completed`
          (`|SpawnActorFromClass` "/Game/FlexibleCombatSystem/Blueprints/Weapons/Projectiles/RadialForce_Bp.RadialForce_Bp_C" (`KismetMathLibrary.MakeTransform` (`self.K2_GetActorLocation` OtherActor)) "Undefined" "OverrideRootScale" null null)
          (`KismetSystemLibrary.Delay` 3.0)
          (goto _label_4 :!via `Reset`)))
      (else
        (set `self.Blocking Hit` false)))))

(fn `ApplyForceDamage`
  (params (BaseDamage :type "Float (single-precision)") (HitInfo :type "HitResult Structure (by ref)") (DamagedActor :type "Actor Object Reference") (HitFromDirection :type "Vector Structure (by ref)"))
  (`GameplayStatics.ApplyPointDamage` DamagedActor BaseDamage HitFromDirection HitInfo null (cast `/Game/FlexibleCombatSystem/Blueprints/BP_PlayerCharacter` (`GameplayStatics.GetPlayerCharacter` 0) :!pure true)))

(fn `Bound by Law`)

(fn `Divine Vigor`)

(fn `Judgment`
  (set `self.UltiC` 1.0)
  (set `self.ActivatedUlti` true))

(fn `JusticaforAll`
  (if (and (<= (`self.Health`) 150) (> (`self.MaxHealth`) 200))
    (set `self.Health` (* (- (`self.MaxHealth`) (`self.Health`)) (/ (`KismetStringLibrary.Conv_StringToInt` "80") 100)))
    (else
      (set `self.Health` 200))))

(fn `Out Range Move`
  (params (CustomRange :type "Float (double-precision)"))
  (`self.SetRotation` (`self.CachedDestination`))
  (`self.MoveTo` (+ (* (- (`self.TargetDistance`) CustomRange) (`KismetMathLibrary.GetForwardVector` (`self.K2_GetActorRotation`))) (`self.K2_GetActorLocation`))))

(fn `Purge Evil`)

(fn `Reciprocate`
  (set `self.MainLevelDamage` 190))

(fn `Salvation`
  (if (and (<= (`self.Health`) 150) (> (`self.MaxHealth`) 200))
    (set `self.Health` (+ (`self.Health`) 140))
    (else
      (set `self.Health` 200))))

(fn `Sanctification`)

(fn `SetRotation`
  (params (To :type "Vector Structure"))
  (bind (_returnvalue_roll _returnvalue_pitch _returnvalue_yaw) (`KismetMathLibrary.BreakRotator` (`KismetMathLibrary.Conv_VectorToRotator` (`KismetMathLibrary.GetDirectionUnitVector` (`self.K2_GetActorLocation`) To))))
  (`self.K2_SetActorRotation` (`KismetMathLibrary.MakeRotator` _returnvalue_roll 0.0 _returnvalue_yaw)))

(fn `Stalwart Angel`
  (set `self.Gain25Armor` true))

(fn `Swift Retribution`
  (params (`In Play Rate` :type "Float (single-precision)") (`Max Walk Speed` :type "Float (single-precision)"))
  (set `self.In Play Rate` `In Play Rate`)
  (set `CharacterMovementComponent.MaxWalkSpeed` `Max Walk Speed` (`self.CharacterMovement`)))

(fn `UpgradeLevel`
  (bind _levelsystem_comp (`self.LevelSystem_Comp`))
  (if (== (`self.TotalLevel`) 1)
    (set `/Game/UI/Blueprint/LevelSystem_Comp.Levels` "NewEnumerator0" _levelsystem_comp)
    (return)
    (elif (== (`self.TotalLevel`) 2)
      (set `/Game/UI/Blueprint/LevelSystem_Comp.Levels` "NewEnumerator1" _levelsystem_comp)
      (return)
      (elif (== (`self.TotalLevel`) 3)
        (set `/Game/UI/Blueprint/LevelSystem_Comp.Levels` "NewEnumerator2" _levelsystem_comp)
        (return)
        (elif (>= (`self.TotalLevel`) 4)
          (set `/Game/UI/Blueprint/LevelSystem_Comp.Levels` "NewEnumerator3" _levelsystem_comp)
          (return))))))

(fn `UserConstructionScript`
  (`parent.UserConstructionScript`))
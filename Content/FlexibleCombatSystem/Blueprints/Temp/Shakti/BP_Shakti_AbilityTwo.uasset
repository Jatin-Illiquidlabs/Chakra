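; Playable mage character Shakti with cursor-targeted abilities: ability keys arm an ability, Select casts it, Cancel clears it.
; Casts cover a triple projectile from three arrow components, a montage attack with move-into-range, a range-limited teleport, and a timed ultimate that tracks the cursor.
; Tick aims and debug-traces the arrows during Ability1 targeting and maps TotalLevel onto LevelSystemComp.
; BeginPlay adds the level-up widget; the named skill functions are empty stubs.
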(event `self.ReceiveTick`
  (params (DeltaSeconds :type "Float (single-precision)"))
  (bind (_hit _location) (`self.GetLocationUnderCursor`))
  (bind _arrow1 (`self.Arrow1`))
  (`parent.ReceiveTick` DeltaSeconds)
  (`|ExecutionSequence`
    (:`then_0`
      (if (`|EnumEquality` (`self.AbilityType`) "NewEnumerator0")
        (`SceneComponent.SetHiddenInGame` _arrow1 false false)
        (`SceneComponent.SetHiddenInGame` (`self.Arrow3`) false false)
        (`SceneComponent.SetHiddenInGame` (`self.Arrow2`) false false)
        (if (not (and (`self.IsAttacking`) (not (`self.UltiActivated`))))
          (bind _output_get (set `self.CachedDestination` (`.Location` (`self.GetLocationUnderCursor`)))))
        (bind (_returnvalue_roll _returnvalue_pitch _returnvalue_yaw) (`KismetMathLibrary.BreakRotator` (`KismetMathLibrary.FindLookAtRotation` (`self.K2_GetActorLocation`) _output_get)))
        (`SceneComponent.K2_SetWorldRotation` (`self.Arrow2`) (`KismetMathLibrary.MakeRotator` 0.0 0.0 _returnvalue_yaw) false false)
        (`SceneComponent.K2_SetWorldRotation` (`self.Arrow1`) (`KismetMathLibrary.MakeRotator` 0.0 0.0 _returnvalue_yaw) false false)
        (`SceneComponent.K2_SetWorldRotation` (`self.Arrow3`) (`KismetMathLibrary.MakeRotator` 0.0 0.0 _returnvalue_yaw) false false)
        (bind _output_get_2 (set `self.CachedDestination` _output_get))
        (bind _returnvalue (+ (.z _output_get_2) 120.0))
        (`self.TraceArrow` (`self.Arrow2`) (`KismetMathLibrary.MakeVector` (.x _output_get_2) (.y _output_get_2) _returnvalue))
        (`self.TraceArrow` (`self.Arrow1`) (`KismetMathLibrary.MakeVector` (.x _output_get_2) (.y _output_get_2) _returnvalue))
        (`self.TraceArrow` (`self.Arrow3`) (`KismetMathLibrary.MakeVector` (.x _output_get_2) (.y _output_get_2) _returnvalue))
        (else
          (`SceneComponent.SetHiddenInGame` _arrow1 true false)
          (`SceneComponent.SetHiddenInGame` (`self.Arrow3`) true false)
          (`SceneComponent.SetHiddenInGame` (`self.Arrow2`) true false)))
      (if (`self.UltiOnePose`)
        (set `self.CachedDestination` _location)
        (`self.SetRotation` _location)))
    (:`then_1`
      (`self.UpgradeLevel`))))

(event `InputVectorAxis|Mouse2D`
  (params (AxisValue :type "Vector Structure"))
  (if (> (`KismetMathLibrary.Vector_GetAbsMax` AxisValue) 0.0)
    _))

(event `InputAction|CancelAbility`
  (params (Key :type "Key Structure"))
  ;[0.9685 0.9571 1] Abilities
  ;;[1 0 0] Cancel
  (:`Pressed`
    (if (and (`self.SelecetedPoint`) (not (`self.IsAttacking`)))
      (set `self.SelecetedPoint` false)
      (set `PlayerController.CurrentMouseCursor` "Default" (`GameplayStatics.GetPlayerController` 0))
      (set `self.AbleToAttack` true)
      (set `self.AbilityType` "NewEnumerator4"))))

(event `self.ReceiveBeginPlay`
  (bind _returnvalue (`|CreateWidget` "/Game/UI/LevelUp_Widget_Mage.LevelUp_Widget_Mage_C"))
  (`UserWidget.AddToViewport` _returnvalue 0))

(event `InputAction|Ability1`
  (params (Key :type "Key Structure"))
  ;[0.9685 0.9571 1] Abilities
  (:`Pressed`
    (`self.StopMovementController`)
    (set `self.SelecetedPoint` true)
    (set `self.AbilityType` "NewEnumerator0")
    (set `PlayerController.CurrentMouseCursor` "Hand" (`GameplayStatics.GetPlayerController` 0))))

(event `InputAction|Ability2`
  (params (Key :type "Key Structure"))
  ;[0.9685 0.9571 1] Abilities
  (:`Pressed`
    (`self.StopMovementController`)
    (set `self.SelecetedPoint` true)
    (set `self.AbilityType` "NewEnumerator1")
    (set `PlayerController.CurrentMouseCursor` "Hand" (`GameplayStatics.GetPlayerController` 0))))

(event `InputAction|Ability3`
  (params (Key :type "Key Structure"))
  ;[0.9685 0.9571 1] Abilities
  (:`Pressed`
    (`self.StopMovementController`)
    (set `self.SelecetedPoint` true)
    (set `self.AbilityType` "NewEnumerator2")
    (set `PlayerController.CurrentMouseCursor` "Hand" (`GameplayStatics.GetPlayerController` 0))))

(event `InputAction|Hero Ability`
  (params (Key :type "Key Structure"))
  ;[0.9685 0.9571 1] Abilities
  (:`Pressed`
    (`self.StopMovementController`)
    (set `self.SelecetedPoint` true)
    (set `self.AbilityType` "NewEnumerator3")
    (set `PlayerController.CurrentMouseCursor` "Hand" (`GameplayStatics.GetPlayerController` 0))))

(event `InputAction|Select`
  (params (Key :type "Key Structure"))
  (bind _returnvalue (`KismetMathLibrary.Vector_Distance` (`self.CachedDestination`) (`self.K2_GetActorLocation`)))
  (bind _returnvalue_2 (`KismetMathLibrary.Vector_Distance` (`self.CachedDestination`) (`self.K2_GetActorLocation`)))
  (bind _returnvalue_3 (`KismetMathLibrary.Vector_Distance` (`self.CachedDestination`) (`self.K2_GetActorLocation`)))
  ;[0.9685 0.9571 1] Abilities
  (:`Pressed`
    (if (`self.SelecetedPoint`)
      (bind _output_get (set `self.CachedDestination` (`.Location` (`self.GetLocationUnderCursor`))))
      (switch `/Game/FlexibleCombatSystem/Blueprints/PaladinChar_AbilityType` (`self.AbilityType`)
        (:`NewEnumerator0`
          (`/Engine/EditorBlueprintResources/StandardMacros.DoOnce` false :!label _label
            (:`Completed`
              (if (`self.IsAttacking`)
                (goto _label :!via `Reset`)
                (else
                  (set `self.IsAttacking` true)
                  (set `self.AbleToAttack` false)
                  (bind _output_get_2 (set `self.Current Anim Montage` "/Game/Characters/RevizedAnimations/ShaktiAnims/Shakti_AbilityOneMontage.Shakti_AbilityOneMontage"))
                  (`self.PlayAnimMontage` _output_get_2)
                  (`self.SetRotation` _output_get)
                  (set `PlayerController.CurrentMouseCursor` "Default" (`GameplayStatics.GetPlayerController` 0))
                  (set `self.SelecetedPoint` false)
                  (`KismetSystemLibrary.Delay` 0.4)
                  (`self.SpawnTripleProjetile` _output_get _output_get _output_get)
                  (set `self.AbleToAttack` true)
                  (set `self.AbilityType` "NewEnumerator4")
                  (goto _label :!via `Reset`))))))
        (:`NewEnumerator1`
          (`/Engine/EditorBlueprintResources/StandardMacros.DoOnce` false :!label _label_2
            (:`Completed`
              (if (`self.IsAttacking`)
                (goto _label_2 :!via `Reset`)
                (else
                  (set `self.IsAttacking` true)
                  (set `self.AbleToAttack` false)
                  (set `self.TargetDistance` _returnvalue_3)
                  (if (<= _returnvalue_3 1200.0)
                    (bind _output_get_3 (set `self.Current Anim Montage` "/Game/Characters/RevizedAnimations/ShaktiAnims/Shakti_AbilityTwoMobtage.Shakti_AbilityTwoMobtage"))
                    (else
                      (`self.Out Range Move` 600.0)
                      (`KismetSystemLibrary.Delay` 2.0)))
                  (`self.PlayAnimMontage` _output_get_3)
                  (`self.SetRotation` _output_get)
                  (set `PlayerController.CurrentMouseCursor` "Default" (`GameplayStatics.GetPlayerController` 0))
                  (set `self.SelecetedPoint` false)
                  (set `self.AbleToAttack` true)
                  (set `self.AbilityType` "NewEnumerator4")
                  (goto _label_2 :!via `Reset`))))))
        (:`NewEnumerator2`
          (`/Engine/EditorBlueprintResources/StandardMacros.DoOnce` false :!label _label_3
            (:`Completed`
              (set `self.TargetDistance` _returnvalue_2)
              (set `self.AbleToAttack` false)
              (if (<= _returnvalue_2 700.0)
                (`self.K2_TeleportTo` _output_get)
                (`NiagaraFunctionLibrary.SpawnSystemAtLocation` "/Game/Plugins/DarkSocerer_Animset/demo/FX/NS_FireToon.NS_FireToon" _output_get)
                (`self.SetRotation` _output_get)
                (set `self.SelecetedPoint` false)
                (set `PlayerController.CurrentMouseCursor` "Default" (`GameplayStatics.GetPlayerController` 0))
                (set `self.AbleToAttack` true)
                (set `self.AbilityType` "NewEnumerator4")
                (goto _label_3 :!via `Reset`)
                (else
                  (goto _label_3 :!via `Reset`))))))
        (:`NewEnumerator3`
          (`/Engine/EditorBlueprintResources/StandardMacros.DoOnce` false :!label _label_4
            (:`Completed`
              (if (`self.IsAttacking`)
                (goto _label_4 :!via `Reset`)
                (else
                  (set `self.IsAttacking` true)
                  (set `self.TargetDistance` _returnvalue)
                  (if (<= _returnvalue 1200.0)
                    (set `self.UltiActivated` true)
                    (set `self.AbleToAttack` false)
                    (bind _output_get_4 (set `self.Current Anim Montage` "/Game/Characters/RevizedAnimations/ShaktiAnims/Shakti_UltiStartMontage.Shakti_UltiStartMontage"))
                    (bind _returnvalue_4 (`self.PlayAnimMontage` _output_get_4))
                    (`KismetSystemLibrary.Delay` _returnvalue_4)
                    (set `self.UltiOnePose` true)
                    (`KismetSystemLibrary.Delay` 3.0)
                    (set `self.UltiOnePose` false)
                    (set `self.UltiActivated` false)
                    (bind _output_get_5 (set `self.Current Anim Montage` "/Game/Characters/RevizedAnimations/ShaktiAnims/Shakti_UltiEndMontage.Shakti_UltiEndMontage"))
                    (bind _returnvalue_5 (`self.PlayAnimMontage` _output_get_5))
                    (`KismetSystemLibrary.Delay` _returnvalue_5)
                    (set `self.SelecetedPoint` false)
                    (set `PlayerController.CurrentMouseCursor` "Default" (`GameplayStatics.GetPlayerController` 0))
                    (set `self.AbleToAttack` true)
                    (set `self.AbilityType` "NewEnumerator4")
                    (set `self.IsAttacking` false)
                    (goto _label_4 :!via `Reset`)))))))))))

(fn `Aether Walker`)

(fn `Calamity`)

(fn `ChargedBlast`)

(fn `Disintegrate`)

(fn `Dominance`)

(fn `Force Armor`)

(fn `Out Range Move`
  (params (CustomRange :type "Float (double-precision)"))
  (`self.SetRotation` (`self.CachedDestination`))
  (`self.MoveTo` (+ (* (- (`self.TargetDistance`) CustomRange) (`KismetMathLibrary.GetForwardVector` (`self.K2_GetActorRotation`))) (`self.K2_GetActorLocation`))))

(fn `PowerHungry`)

(fn `SetRotation`
  (params (To :type "Vector Structure"))
  (bind (_returnvalue_roll _returnvalue_pitch) (`KismetMathLibrary.BreakRotator` (`self.K2_GetActorRotation`)))
  (bind (_returnvalue_roll_2 _returnvalue_pitch_2 _returnvalue_yaw) (`KismetMathLibrary.BreakRotator` (`KismetMathLibrary.Conv_VectorToRotator` (`KismetMathLibrary.GetDirectionUnitVector` (`self.K2_GetActorLocation`) To))))
  (`self.K2_SetActorRotation` (`KismetMathLibrary.MakeRotator` _returnvalue_roll _returnvalue_pitch _returnvalue_yaw)))

(fn `Skeer`)

(fn `SpawnPorjectileAbility`
  (params (InSocketName :type Name) (Class :type "Actor Class Reference") (Target :type "SceneComponent Object Reference") (`Spawn Transform Rotation` :type "Rotator Structure"))
  (bind _returnvalue (`SceneComponent.GetSocketLocation` Target InSocketName))
  (bind _mesh (`self.Mesh`))
  (`|ExecutionSequence`
    (:`then_0`
      (`GameplayStatics.SpawnEmitterAtLocation` "/Game/DarkSocerer_Animset/demo/FX/P_Hit.P_Hit" _returnvalue))
    (:`then_1`
      (bind _returnvalue_2 (`|SpawnActorFromClass` Class (`KismetMathLibrary.MakeTransform` _returnvalue `Spawn Transform Rotation`) "Undefined" "OverrideRootScale" null null))
      (set `self.SpawnProjectile` _returnvalue_2)
      (`GameplayStatics.SpawnEmitterAttached` null _mesh (`SkinnedMeshComponent.GetSocketBoneName` _mesh "hand_r") (0.0 0.0 0.0) (struct) (0.3 0.3 0.3))
      (`self.CameraShake`))))

(fn `SpawnTripleProjetile`
  (params (A :type "Vector Structure") (A2 :type "Vector Structure") (A3 :type "Vector Structure"))
  (bind _arrow2 (`self.Arrow2`))
  (bind _arrow1 (`self.Arrow1`))
  (bind _arrow3 (`self.Arrow3`))
  (bind (_returnvalue_roll _returnvalue_pitch _returnvalue_yaw) (`KismetMathLibrary.BreakRotator` (`KismetMathLibrary.MakeRotFromX` (- A (`SceneComponent.K2_GetComponentLocation` _arrow1)))))
  (bind (_returnvalue_roll_2 _returnvalue_pitch_2 _returnvalue_yaw_2) (`KismetMathLibrary.BreakRotator` (`KismetMathLibrary.MakeRotFromX` (- A2 (`SceneComponent.K2_GetComponentLocation` _arrow2)))))
  (bind (_returnvalue_roll_3 _returnvalue_pitch_3 _returnvalue_yaw_3) (`KismetMathLibrary.BreakRotator` (`KismetMathLibrary.MakeRotFromX` (- A3 (`SceneComponent.K2_GetComponentLocation` _arrow3)))))
  (`|ExecutionSequence`
    (:`then_0`
      (`self.SpawnPorjectileAbility` "None" "/Game/FlexibleCombatSystem/Blueprints/Weapons/Projectiles/BP_TripleProjectile.BP_TripleProjectile_C" _arrow1 (`KismetMathLibrary.MakeRotator` _returnvalue_roll 0.0 _returnvalue_yaw)))
    (:`then_1`
      (`self.SpawnPorjectileAbility` "None" "/Game/FlexibleCombatSystem/Blueprints/Weapons/Projectiles/BP_TripleProjectile.BP_TripleProjectile_C" _arrow2 (`KismetMathLibrary.MakeRotator` _returnvalue_roll_2 0.0 _returnvalue_yaw_2)))
    (:`then_2`
      (`self.SpawnPorjectileAbility` "None" "/Game/FlexibleCombatSystem/Blueprints/Weapons/Projectiles/BP_TripleProjectile.BP_TripleProjectile_C" _arrow3 (`KismetMathLibrary.MakeRotator` _returnvalue_roll_3 0.0 _returnvalue_yaw_3)))))

(fn `TraceArrow`
  (params (Target :type "SceneComponent Object Reference") (End :type "Vector Structure"))
  (`KismetSystemLibrary.LineTraceMultiForObjects` :`Start` (`SceneComponent.GetSocketLocation` Target "None") :`End` End :`ObjectTypes` (`|MakeArray` "ObjectTypeQuery1" :!type "EObjectTypeQuery Enum") :`DrawDebugType` "ForOneFrame"))

(fn `Triumvirate`)

(fn `UpgradeLevel`
  (bind _levelsystem_comp (`self.LevelSystem_Comp`))
  (if (== (`self.TotalLevel`) 1)
    (set `/Game/UI/Blueprint/LevelSystem_Comp.Levels` "NewEnumerator0" _levelsystem_comp)
    (return)
    (elif (== (`self.TotalLevel`) 2)
      (set `/Game/UI/Blueprint/LevelSystem_Comp.Levels` "NewEnumerator1" _levelsystem_comp)
      (return)
      (elif (== (`self.TotalLevel`) 3)
        (set `/Game/UI/Blueprint/LevelSystem_Comp.Levels` "NewEnumerator2" _levelsystem_comp)
        (return)
        (elif (== (`self.TotalLevel`) 4)
          (set `/Game/UI/Blueprint/LevelSystem_Comp.Levels` "NewEnumerator2" _levelsystem_comp)
          (return))))))

(fn `UserConstructionScript`
  (`parent.UserConstructionScript`))

(fn `Wave of Force`)

(fn `Zei's Vengeance`)
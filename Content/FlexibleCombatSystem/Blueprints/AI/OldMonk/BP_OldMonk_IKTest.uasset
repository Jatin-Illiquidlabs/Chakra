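; BP_OldMonk_IKTest is a test Blueprint for the Old Monk AI that gathers hand IK data from the environment.
; Every Tick, IKHandTrace casts a debug-drawn Visibility line trace from the left and right hand sockets along the actor's downward axis.
; Each trace stores a hit location and a hit flag per hand, zeroing the location on a miss; despite the "HitWall" naming, it only probes downward.
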(event `self.ReceiveTick`
  (params (DeltaSeconds :type "Float (single-precision)"))
  (`|ExecutionSequence`
    (:`then_0`
      (bind (_hitlocation _hashitwall) (`self.IKHandTrace` "Hand_L" 100.0))
      (set `self.IKLeftHandLocation` _hitlocation)
      (set `self.LeftHandHitWall` _hashitwall))
    (:`then_1`
      (bind (_hitlocation_2 _hashitwall_2) (`self.IKHandTrace` "Hand_R" 100.0))
      (set `self.IKRightHandLocation` _hitlocation_2)
      (set `self.RightHandHitWall` _hashitwall_2))))

(fn `IKHandTrace`
  (params (SocketName :type Name) (Distance :type "Float (double-precision)"))
  (returns (HitLocation :type "Vector Structure") (HasHitWall :type Boolean))
  (bind _returnvalue (`SceneComponent.GetSocketLocation` (`self.Mesh`) SocketName))
  (bind (_outhit _returnvalue_2) (`KismetSystemLibrary.LineTraceSingle` :`Start` _returnvalue :`End` (+ _returnvalue (* (* (`self.GetActorUpVector`) -1) Distance)) :`TraceChannel` "TraceTypeQuery1" :`DrawDebugType` "ForOneFrame"))
  (if _returnvalue_2
    (return (`.Location` (`GameplayStatics.BreakHitResult` _outhit)) true)
    (else
      (return (0.0 0.0 0.0) false))))

(fn `UserConstructionScript`)
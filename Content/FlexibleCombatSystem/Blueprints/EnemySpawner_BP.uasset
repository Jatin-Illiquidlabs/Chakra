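; EnemySpawner_BP is a spawner that keeps producing AI enemies at its own location during play.
; After an initial delay on BeginPlay, a looping timed Delay calls SpawnMinion repeatedly, with no count limit or stop condition.
; SpawnMinion uses SpawnAIFromClass to create a BP_EnemyAI running BT_AI, rotated to face the first player's pawn.
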(event `self.ReceiveBeginPlay`
  (`KismetSystemLibrary.Delay` 20.0)
  (`self.SpawnMinion` :!label _label)
  (`KismetSystemLibrary.Delay` 5.0)
  (goto _label))

(event `SpawnMinion`
  (`AIBlueprintHelperLibrary.SpawnAIFromClass` "/Game/FlexibleCombatSystem/Blueprints/AI/BP_EnemyAI.BP_EnemyAI_C" "/Game/FlexibleCombatSystem/Blueprints/AI/BT_AI.BT_AI" (`self.K2_GetActorLocation`) (`KismetMathLibrary.MakeRotFromX` (- (`self.K2_GetActorLocation` (`GameplayStatics.GetPlayerPawn` 0)) (`self.K2_GetActorLocation`))) false null))

(fn `UserConstructionScript`)
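; Base pickup item actor that launches upward with an aura trail and sound, then is collected by the player.
; SetItemVFX, called on BeginPlay with Uncommon assets, sets the effects and launches physics-simulated collision and mesh.
; Tick keeps the collision's world rotation zeroed, and a collision hit stops both simulations.
; Player overlap on the mesh calls PickupAbility, which spawns pickup FX, then destroys the actor.
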(event `self.ReceiveBeginPlay`
  (`self.Set Item VFX` "/Game/Vefects/Item_Pickup_VFX/Shared/Particles/NS_ItemAura_Uncommon.NS_ItemAura_Uncommon" "/Game/Vefects/Item_Pickup_VFX/Audio/SND_Item_Uncommon_L.SND_Item_Uncommon_L"))

(event `PickupAbility`
  (params (PlayerCharacter :type "/Game/FlexibleCombatSystem/Blueprints/BP_PlayerCharacter Object Reference"))
  (`NiagaraFunctionLibrary.SpawnSystemAtLocation` (`self.PickupItemFX`) (`SceneComponent.K2_GetComponentLocation` (`self.StaticMesh`))))

(event `self.StaticMesh.OnComponentBeginOverlap`
  (params (OverlappedComponent :type "PrimitiveComponent Object Reference") (OtherActor :type "Actor Object Reference") (OtherComp :type "PrimitiveComponent Object Reference") (OtherBodyIndex :type Integer) (bFromSweep :type Boolean) (SweepResult :type "HitResult Structure (by ref)"))
  (bind _asbp_player_character (cast `/Game/FlexibleCombatSystem/Blueprints/BP_PlayerCharacter` OtherActor))
  (`self.PickupAbility` _asbp_player_character)
  (`self.K2_DestroyActor`))

(event `Set Item VFX`
  (params (Trail :type "NiagaraSystem Object Reference") (SFX :type "SoundBase Object Reference"))
  (bind _collision (`self.Collision`))
  (bind _staticmesh (`self.StaticMesh`))
  ;[0.7478 1 0.2155] Set up Item
  (`NiagaraComponent.SetAsset` (`self.TrailVFX`) Trail true)
  (`AudioComponent.SetSound` (`self.Audio`) SFX)
  (`PrimitiveComponent.SetSimulatePhysics` _collision true)
  (`PrimitiveComponent.SetAllPhysicsLinearVelocity` _collision (0.0 0.0 500.0) false)
  (`PrimitiveComponent.SetSimulatePhysics` _staticmesh true)
  (`PrimitiveComponent.SetAllPhysicsLinearVelocity` _staticmesh (0.0 0.0 500.0) false))

(event `self.ReceiveTick`
  (params (DeltaSeconds :type "Float (single-precision)"))
  (`SceneComponent.K2_SetWorldRotation` :`self` (`self.Collision`)))

(event `self.Collision.OnComponentHit`
  (params (HitComponent :type "PrimitiveComponent Object Reference") (OtherActor :type "Actor Object Reference") (OtherComp :type "PrimitiveComponent Object Reference") (NormalImpulse :type "Vector Structure") (Hit :type "HitResult Structure (by ref)"))
  (`PrimitiveComponent.SetSimulatePhysics` (`self.Collision`) false)
  (`PrimitiveComponent.SetSimulatePhysics` (`self.StaticMesh`) false))

(fn `UserConstructionScript`)
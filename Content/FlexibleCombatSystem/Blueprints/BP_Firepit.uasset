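; BP_Firepit is an actor that moves its static mesh back and forth along a spline.
; On BeginPlay it waits a random delay and sets a random timeline play rate, varying timing between instances.
; The timeline maps its Distance track onto spline length to position the mesh without sweep, then flips direction on finish and replays forward or reversed.
; A tangent-based rotation node exists but is never executed.
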(event `self.ReceiveBeginPlay`
  (`KismetSystemLibrary.Delay` (`KismetMathLibrary.RandomFloatInRange` 0.0 2.0))
  (set `self.TimelineLength` (`KismetMathLibrary.RandomFloatInRange` 0.3 1.0))
  (`TimelineComponent.SetPlayRate` (`self.Firepit_Timeline`) (`self.TimelineLength`))
  (`self.StartMovement` (`self.IsMovingForward`)))

(event `StartMovement`
  (params (IsMovingForward :type Boolean))
  (bind _spline (`self.Spline`))
  (if IsMovingForward
    (bind (_direction _distance) (`Timeline|Firepit_Timeline` :!via `PlayFromStart` :!label _label)
      (:`Update`
        (`SceneComponent.K2_SetWorldLocation` (`self.StaticMesh`) (`SplineComponent.GetLocationAtDistanceAlongSpline` (`self.Spline`) (`KismetMathLibrary.Lerp` 0.0 (`SplineComponent.GetDistanceAlongSplineAtSplinePoint` _spline (- (`SplineComponent.GetNumberOfSplinePoints` _spline) 1)) _distance) "World") false false))
      (:`Finished`
        (bind _output_get (set `self.IsMovingForward` (not (`self.IsMovingForward`))))
        (set `self.SplineIndex` (* (`self.SplineIndex`) -1))
        (`self.StartMovement` _output_get)))
    (else
      (goto _label :!via `ReverseFromEnd`))))

(fn `UserConstructionScript`)
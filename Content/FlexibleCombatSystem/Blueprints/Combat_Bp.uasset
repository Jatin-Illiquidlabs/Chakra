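; Combat component that handles buffered action input, action state, melee hit detection and hit reactions for its owning character.
; Input is stored and consumed when nothing is executing, routing to an empty Light Attack stub or an Interaction state.
; While attacking, Tick box-traces around the spine socket, calling GetHit once per new target that has this component.
; GetHit plays a delayed stun montage; helpers temporarily ignore root motion during movement input.
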(event `TraceOn`
  (params (AttackType :type Byte :default 0) (`RightHand?` :type Boolean) (`Trace?` :type Boolean))
  ;[0.4844 0.1718 0.07147] TraceAction
  (set `self.TraceOn?` `Trace?`)
  (`KismetArrayLibrary.Array_Clear` (`self.EnemyToHit`)))

(event `self.ReceiveTick`
  (params (DeltaSeconds :type "Float (single-precision)"))
  (if (`self.Attack?`)
    (`self.PerformTrace`)))

(event `PerformTrace`
  (bind _enemytohit (`self.EnemyToHit`))
  ;[0.4844 0.1718 0.07147] TraceAction
  (bind (_outhits _returnvalue) (`self.SelectAttackTrace`))
  (if _returnvalue
    (for _array_element _outhits
      (bind (_bblockinghit _binitialoverlap _time _distance _location _impactpoint _normal _impactnormal _physmat _hitactor) (`GameplayStatics.BreakHitResult` _array_element))
      (`/Engine/EditorBlueprintResources/StandardMacros.IsValid` (`self.GetCombatClass` _hitactor)
        (:`Is Valid`
          (if (not (`KismetArrayLibrary.Array_Contains` _enemytohit _hitactor))
            (`KismetArrayLibrary.Array_Add` _enemytohit _hitactor)
            (bind (_returnvalue_2 _attacker _target) (`self.CalculateReaction` _hitactor))
            (`self.GetHit` _returnvalue_2 _target)))))))

(event `ActionInput`
  (params (`Attack Move` :type "/Game/FlexibleCombatSystem/Blueprints/Data/E_AttackMove Enum" :default "NewEnumerator0"))
  (set `self.StoredKey` `Attack Move`)
  (if (not (`self.Executing`))
    (`self.QueueInput`)))

(event `Consumed Key`
  (params (`Attack Move` :type "/Game/FlexibleCombatSystem/Blueprints/Data/E_AttackMove Enum" :default "NewEnumerator0"))
  (switch `/Game/FlexibleCombatSystem/Blueprints/Data/E_AttackMove` `Attack Move`
    (:`NewEnumerator1`
      (`self.Light Attack`))
    (:`NewEnumerator3`
      (`self.SetState` "NewEnumerator3" true))))

(event `GetHit`
  (params (HitReaction :type "/Game/FlexibleCombatSystem/Blueprints/GetHit Structure"))
  ;[0.4844 0.1718 0.07147] TraceAction
  (`KismetSystemLibrary.Delay` 1.0)
  (`AnimInstance.Montage_Play` (`self.AnimInstance`) (`.Stun_2_7A3E741945474FDC1140D59351FFA2E9` (break `/Game/FlexibleCombatSystem/Blueprints/GetHit` HitReaction)) 1.0 "MontageLength" 0.0 true))

(event `Initialize`
  (params (CaharacterMovement :type "CharacterMovementComponent Object Reference") (Mesh :type "SkeletalMeshComponent Object Reference") (AnimInstance :type "SkeletalMeshComponent Object Reference"))
  (`self.CalculateVeriable` CaharacterMovement Mesh AnimInstance))

(fn `Enable Root Motion`
  (`AnimInstance.SetRootMotionMode` (`self.AnimInstance`) "RootMotionFromMontagesOnly"))

(fn `Executed`
  (`self.SetState` "NewEnumerator0" true)
  (set `self.Attacking` false))

(fn `GetCombatClass`
  (params (self2 :type "Actor Object Reference"))
  (returns (ReturnValue :type "/Game/FlexibleCombatSystem/Blueprints/Combat_Bp Object Reference"))
  (return (`Actor.GetComponentByClass` self2 "Combat_Bp_C")))

(fn `IgnoreRootMotion`
  (if (!= (`PawnMovementComponent.GetLastInputVector` (`self.CharacterMovement`)) (0.0 0.0 0.0))
    (`AnimInstance.SetRootMotionMode` (`self.AnimInstance`) "IgnoreRootMotion")
    (`KismetSystemLibrary.K2_SetTimer` null "Enable Root Motion" 0.32)))

(fn `Light Attack`)

(fn `QueueInput`
  (`self.Consumed Key` (`self.StoredKey`))
  (set `self.StoredKey` "NewEnumerator0"))

(fn `SelectAttackTrace`
  (returns (OutHits :type "Array of HitResult Structure") (ReturnValue :type Boolean))
  (bind _mesh (`self.Mesh`))
  ;[0.1099 0 1] Axe
  (bind (_outhits _returnvalue) (`KismetSystemLibrary.BoxTraceMultiForObjects` (`SceneComponent.GetSocketLocation` _mesh "spine_01") (`SceneComponent.GetSocketLocation` _mesh "spine_01") (300.0 300.0 300.0) (`SceneComponent.GetSocketRotation` _mesh "spine_01") (`|MakeArray` "ObjectTypeQuery8" :!type "EObjectTypeQuery Enum") false (`|MakeArray` (`self.GetOwner`)) "ForOneFrame"))
  (return _outhits _returnvalue))

(fn `SetState`
  (params (State :type "/Game/FlexibleCombatSystem/Blueprints/Data/E_ActiveState Enum" :default "NewEnumerator0") (SelectExecution :type Boolean))
  (`/Game/FlexibleCombatSystem/Blueprints/MacroLibrary.ML_SetPreviousAndNewValue` State (`self.ActiveState`) (`self.PreviousState`))
  (if SelectExecution
    (set `self.Executing` (`|EnumInequality` State "NewEnumerator0"))))
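; Gameplay ability for a spell attack that fires projectiles from the avatar during an attack montage.
; On activation it commits, plays a random tagged montage and waits for the FireBolt montage event.
; That event spawns projectiles homing on the combat target, using the montage's socket location at a fixed height as target location.
; It ends when the montage finishes; an uncalled SetRotaion helper yaws the character toward the projectile target.
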(event `self.K2_ActivateAbility`
  (`KismetSystemLibrary.PrintString` "Hello")
  (`self.K2_CommitAbility`)
  (bind _returnvalue (message `CombatInterface.GetAttackMontages` (`self.GetAvatarActorFromActorInfo`)))
  (bind _output_get (set `self.TaggedMontages` (`self.GetRandomTaggedMontageFromArray` _returnvalue)))
  (bind (_montage _montagetag _sockettag) (break `TaggedMontage` _output_get))
  (`AbilityTask_PlayMontageAndWait.CreatePlayMontageAndWaitProxy` "None" _montage 1.0 "None" false
    (:`then`
      (`AbilityTask_WaitGameplayEvent.WaitGameplayEvent` (struct :`TagName` "Event.Montage.FireBolt") null
        (:`EventReceived`
          (bind _returnvalue_2 (message `CombatInterface.GetCombatSocketLocation` (`self.GetAvatarActorFromActorInfo`) _sockettag))
          (`self.SpawnProjectiles` (`KismetMathLibrary.MakeVector` (.x _returnvalue_2) (.y _returnvalue_2) 45.0) (`BlueprintGameplayTagLibrary.MakeLiteralGameplayTag` (struct :`TagName` "CombatSocket.ArrowsMid")) false 0.0 (`self.CombatTarget`)))))
    (:`OnCompleted`
      (`self.K2_EndAbility` :!label _label))
    (:`OnBlendOut`
      (goto _label))
    (:`OnInterrupted`
      (goto _label))
    (:`OnCancelled`
      (goto _label))))

(fn `SetRotaion`
  (params (Object :type "Object Object Reference"))
  (bind _aschakra_character (cast `ChakraCharacter` Object))
  (bind (_returnvalue_roll _returnvalue_pitch) (`KismetMathLibrary.BreakRotator` (`Actor.K2_GetActorRotation` _aschakra_character)))
  (bind (_returnvalue_roll_2 _returnvalue_pitch_2 _returnvalue_yaw) (`KismetMathLibrary.BreakRotator` (`KismetMathLibrary.Conv_VectorToRotator` (`KismetMathLibrary.GetDirectionUnitVector` (`Actor.K2_GetActorLocation` _aschakra_character) (`self.ProjectileTargetLocation`)))))
  (`Actor.K2_SetActorRotation` _aschakra_character (`KismetMathLibrary.MakeRotator` _returnvalue_roll _returnvalue_pitch _returnvalue_yaw) false))
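; GA_DevaMeleeAttack is a gameplay ability that performs a melee attack with a random montage from the avatar and a trail cue.
; The montage's tagged event triggers a small sphere query at the matching combat socket.
; Non-friendly live players found there receive a damage effect and a blood effect.
; Any hit also fires a MeleeImpact cue, and the ability ends on that event or when the montage completes or is interrupted.
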(event `self.K2_ActivateAbility`
  (bind _returnvalue (`self.GetAvatarActorFromActorInfo`))
  (set `self.HasHitTarget` false)
  (`self.TriggerMeleeAttack`)
  (bind _returnvalue_2 (message `CombatInterface.GetAttackMontages` (`self.GetAvatarActorFromActorInfo`)))
  (bind _output_get (set `self.TaggedMontage` (`self.GetRandomTaggedMontageFromArray` _returnvalue_2)))
  (`self.K2_AddGameplayCue` (struct :`TagName` "GameplayCue.Trail"))
  (bind (_montage _montagetag _sockettag) (break `TaggedMontage` _output_get))
  (`AbilityTask_PlayMontageAndWait.CreatePlayMontageAndWaitProxy` "None" _montage 1.0 "None" false
    (:`then`
      (`AbilityTask_WaitGameplayEvent.WaitGameplayEvent` _montagetag null
        (:`EventReceived`
          (bind _returnvalue_3 (message `CombatInterface.GetCombatSocketLocation` _returnvalue _sockettag))
          (set `self.CombatSocketLocation` _returnvalue_3)
          (bind _outoverlappingactors (`ChakraAbilitySystemLibrary.GetLivePlayersWithinRadius` _returnvalue (`|MakeArray` _returnvalue) 70.0 (`self.CombatSocketLocation`)))
          (for _array_element _outoverlappingactors
            (if (`ChakraAbilitySystemLibrary.IsNotFriend` _array_element (`self.GetAvatarActorFromActorInfo`))
              (`ChakraAbilitySystemLibrary.ApplyDamageEffect` (`self.MakeDamageEffectParamsFromClassDefaults` _array_element))
              (set `self.HasHitTarget` true)
              (message `CombatInterface.GetBloodEffect` _array_element)))
          (if (`self.HasHitTarget`)
            (bind _returnvalue_4 (message `EnemyInterface.GetCombatTarget` (`self.GetAvatarActorFromActorInfo`)))
            (`self.K2_ExecuteGameplayCueWithParams` (struct :`TagName` "GameplayCue.MeleeImpact") (`AbilitySystemBlueprintLibrary.MakeGameplayCueParameters` 0.0 0.0 (struct) (struct) (struct) (`BlueprintGameplayTagLibrary.MakeGameplayTagContainerFromTag` (`.MontageTag` (break `TaggedMontage` (`self.TaggedMontage`)))) (struct) (`self.CombatSocketLocation`) (0.0 0.0 0.0) null (`self.GetAvatarActorFromActorInfo`) _returnvalue_4)))
          (`self.K2_EndAbility`))))
    (:`OnCompleted`
      (`self.K2_EndAbility` :!label _label))
    (:`OnInterrupted`
      (goto _label))
    (:`OnCancelled`
      (goto _label))))
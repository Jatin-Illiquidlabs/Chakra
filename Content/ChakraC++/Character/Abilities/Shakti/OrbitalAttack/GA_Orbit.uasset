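; GA_Orbit is a Shakti gameplay ability that fires projectiles toward the point and actor under the mouse.
; On activation it commits, stores the mouse hit as target and homing actor, updates the avatar's facing and draws a debug sphere.
; An input press then plays the ability montage, whose FireBlast event triggers SpawnProjectiles from a combat socket at a fixed target height.
; The ability ends with the montage; a yaw-facing helper is defined but not called here.
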(event `self.K2_ActivateAbility`
  (bind (_projectiletargetlocation_x _projectiletargetlocation_y) (`KismetMathLibrary.BreakVector` (`self.ProjectileTargetLocation`)))
  (bind (_projectiletargetlocation_x_2 _projectiletargetlocation_y_2 _projectiletargetlocation_z) (`KismetMathLibrary.BreakVector` (`self.ProjectileTargetLocation`)))
  (`self.K2_CommitAbility`)
  (bind (_asynctaskproxy _datahandle) (`TargetDataUnderMouse.CreateTargetDataUnderMouse`)
    (:`ValidData`
      (bind (_bblockinghit _binitialoverlap _time _distance _location _impactpoint _normal _impactnormal _physmat _hitactor) (`GameplayStatics.BreakHitResult` (`AbilitySystemBlueprintLibrary.GetHitResultFromTargetData` _datahandle)))
      (bind _output_get (set `self.ProjectileTargetLocation` (`KismetMathLibrary.MakeVector` (.x _location) (.y _location) (.z _location))))
      (set `self.MouseHitActor` _hitactor)
      (message `CombatInterface.UpdateFacingTarget` (`self.GetAvatarActorFromActorInfo`) (`KismetMathLibrary.MakeVector` _projectiletargetlocation_x_2 _projectiletargetlocation_y_2 _projectiletargetlocation_z))
      (`KismetSystemLibrary.DrawDebugSphere` _output_get 50.0 12 (struct :`R` 0.090903 :`B` 1.0 :`A` 1.0) 3.0 2.0)
      (`AbilityTask_WaitInputPress.WaitInputPress` false
        (:`OnPress`
          (`AbilityTask_PlayMontageAndWait.CreatePlayMontageAndWaitProxy` "None" "/Game/Characters/RevizedAnimations/ShaktiAnims/Shakti_AbilityTwoMobtage.Shakti_AbilityTwoMobtage" 1.0 "None" false
            (:`then`
              (`AbilityTask_WaitGameplayEvent.WaitGameplayEvent` (struct :`TagName` "Event.Montage.FireBlast") null
                (:`EventReceived`
                  (`KismetSystemLibrary.PrintString` "evcent" true true (struct :`R` 1.0 :`G` 0.381075 :`A` 1.0))
                  (`self.SpawnProjectiles` (`KismetMathLibrary.MakeVector` _projectiletargetlocation_x _projectiletargetlocation_y 45.0) (`BlueprintGameplayTagLibrary.MakeLiteralGameplayTag` (struct :`TagName` "CombatSocket.ArrowsMid")) false 0.0 (`self.MouseHitActor`)))))
            (:`OnCompleted`
              (`self.K2_EndAbility` :!label _label))
            (:`OnBlendOut`
              (goto _label))
            (:`OnInterrupted`
              (goto _label))
            (:`OnCancelled`
              (goto _label))))))))

(fn `SetRotaion`
  (params (Object :type "Object Object Reference"))
  (bind _aschakra_character (cast `ChakraCharacter` Object))
  (bind (_returnvalue_roll _returnvalue_pitch) (`KismetMathLibrary.BreakRotator` (`Actor.K2_GetActorRotation` _aschakra_character)))
  (bind (_returnvalue_roll_2 _returnvalue_pitch_2 _returnvalue_yaw) (`KismetMathLibrary.BreakRotator` (`KismetMathLibrary.Conv_VectorToRotator` (`KismetMathLibrary.GetDirectionUnitVector` (`Actor.K2_GetActorLocation` _aschakra_character) (`self.ProjectileTargetLocation`)))))
  (`Actor.K2_SetActorRotation` _aschakra_character (`KismetMathLibrary.MakeRotator` _returnvalue_roll _returnvalue_pitch _returnvalue_yaw) false))
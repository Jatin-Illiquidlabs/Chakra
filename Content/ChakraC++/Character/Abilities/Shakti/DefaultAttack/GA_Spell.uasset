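; GA_Spell is Shakti's default attack gameplay ability, firing homing projectiles at nearby living BP_Zombie actors.
; On activation it commits, scans all zombies without stopping at the first match, and for each in range faces it and plays a random tagged attack montage.
; The montage's gameplay event spawns projectiles from the ArrowsMid socket.
; It ends only on montage cancel; the SetRotaion helper is never called here.
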(event `self.K2_ActivateAbility`
  (bind _returnvalue (`self.GetAvatarActorFromActorInfo`))
  (`KismetSystemLibrary.PrintString` "Hello")
  (`self.K2_CommitAbility`)
  (bind _outactors (`GameplayStatics.GetAllActorsOfClass` "/Game/ChakraC++/Enemy/Zombie/BP_Zombie.BP_Zombie_C"))
  (for _array_element _outactors
    (if (and (< (`Actor.GetDistanceTo` _array_element _returnvalue) 700.0) (not (`ChakraCharacterBase.bDead` _array_element)))
      (`/Engine/EditorBlueprintResources/StandardMacros.IsValid` _array_element
        (:`Is Valid`
          (bind _returnvalue_2 (`Actor.K2_GetActorLocation` _array_element))
          (message `CombatInterface.UpdateFacingTarget` _returnvalue _returnvalue_2)
          (bind _output_get (set `self.NewVar` _returnvalue_2))
          (set `self.CombatTarget` _array_element)
          (bind _returnvalue_3 (message `CombatInterface.GetAttackMontages` (`self.GetAvatarActorFromActorInfo`)))
          (bind _output_get_2 (set `self.TaggedMontages` (`self.GetRandomTaggedMontageFromArray` _returnvalue_3)))
          (bind (_montage _montagetag) (break `TaggedMontage` _output_get_2))
          (`AbilityTask_PlayMontageAndWait.CreatePlayMontageAndWaitProxy` "None" _montage 1.0 "None" false
            (:`then`
              (`AbilityTask_WaitGameplayEvent.WaitGameplayEvent` _montagetag null
                (:`EventReceived`
                  (`KismetSystemLibrary.PrintString` "evcent" true true (struct :`R` 1.0 :`G` 0.381075 :`A` 1.0))
                  (`self.SpawnProjectiles` (`KismetMathLibrary.MakeVector` (.x _output_get) (.y _output_get)) (`BlueprintGameplayTagLibrary.MakeLiteralGameplayTag` (struct :`TagName` "CombatSocket.ArrowsMid")) false 0.0 _array_element))))
            (:`OnCancelled`
              (`self.K2_EndAbility`))))))))

(fn `SetRotaion`
  (params (Object :type "Object Object Reference"))
  (bind _aschakra_character (cast `ChakraCharacter` Object))
  (bind (_returnvalue_roll _returnvalue_pitch) (`KismetMathLibrary.BreakRotator` (`Actor.K2_GetActorRotation` _aschakra_character)))
  (bind (_returnvalue_roll_2 _returnvalue_pitch_2 _returnvalue_yaw) (`KismetMathLibrary.BreakRotator` (`KismetMathLibrary.Conv_VectorToRotator` (`KismetMathLibrary.GetDirectionUnitVector` (`Actor.K2_GetActorLocation` _aschakra_character)))))
  (`Actor.K2_SetActorRotation` _aschakra_character (`KismetMathLibrary.MakeRotator` _returnvalue_roll _returnvalue_pitch _returnvalue_yaw) false))
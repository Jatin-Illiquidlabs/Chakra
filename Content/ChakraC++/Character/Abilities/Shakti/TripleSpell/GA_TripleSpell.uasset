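; Shakti's TripleSpell gameplay ability, which fires projectiles from three arrow sockets toward the point and actor under the mouse.
; On activation it commits, takes mouse target data, draws a debug sphere and sends the avatar a facing update.
; An input press then plays the cast montage, whose FireBlast event spawns the projectiles with the hit actor as homing target.
; The ability ends with the montage; a SetRotaion yaw helper exists but is not called here.
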(event `self.K2_ActivateAbility`
  (bind (_projectiletargetlocation_x _projectiletargetlocation_y _projectiletargetlocation_z) (`KismetMathLibrary.BreakVector` (`self.ProjectileTargetLocation`)))
  (bind (_projectiletargetlocation_x_2 _projectiletargetlocation_y_2 _projectiletargetlocation_z_2) (`KismetMathLibrary.BreakVector` (`self.ProjectileTargetLocation`)))
  (bind (_projectiletargetlocation_x_3 _projectiletargetlocation_y_3 _projectiletargetlocation_z_3) (`KismetMathLibrary.BreakVector` (`self.ProjectileTargetLocation`)))
  (bind (_projectiletargetlocation_x_4 _projectiletargetlocation_y_4 _projectiletargetlocation_z_4) (`KismetMathLibrary.BreakVector` (`self.ProjectileTargetLocation`)))
  (`self.K2_CommitAbility`)
  (bind (_asynctaskproxy _datahandle) (`TargetDataUnderMouse.CreateTargetDataUnderMouse`)
    (:`ValidData`
      (bind (_bblockinghit _binitialoverlap _time _distance _location _impactpoint _normal _impactnormal _physmat _hitactor) (`GameplayStatics.BreakHitResult` (`AbilitySystemBlueprintLibrary.GetHitResultFromTargetData` _datahandle)))
      (bind _output_get (set `self.ProjectileTargetLocation` (`KismetMathLibrary.MakeVector` (.x _location) (.y _location) (.z _location))))
      (`KismetSystemLibrary.DrawDebugSphere` (`KismetMathLibrary.MakeVector` (.x _output_get) (.y _output_get) 45.0) 20.0 12 (struct :`R` 1.0 :`G` 1.0 :`B` 1.0 :`A` 1.0) 3.0 3.0)
      (set `self.MouseHitActor` _hitactor)
      (message `CombatInterface.UpdateFacingTarget` (`self.GetAvatarActorFromActorInfo`) (`KismetMathLibrary.MakeVector` _projectiletargetlocation_x_2 _projectiletargetlocation_y_2 _projectiletargetlocation_z_2))
      (`AbilityTask_WaitInputPress.WaitInputPress` false
        (:`OnPress`
          (`AbilityTask_PlayMontageAndWait.CreatePlayMontageAndWaitProxy` "None" "/Game/Characters/RevizedAnimations/ShaktiAnims/Shakti_AbilityOneMontage.Shakti_AbilityOneMontage" 1.0 "None" false
            (:`then`
              (`AbilityTask_WaitGameplayEvent.WaitGameplayEvent` (struct :`TagName` "Event.Montage.FireBlast") null
                (:`EventReceived`
                  (`self.SpawnProjectiles` (`KismetMathLibrary.MakeVector` _projectiletargetlocation_x_4 _projectiletargetlocation_y_4 _projectiletargetlocation_z_4) (`BlueprintGameplayTagLibrary.MakeLiteralGameplayTag` (struct :`TagName` "CombatSocket.ArrowsMid")) false 0.0 (`self.MouseHitActor`))
                  (`self.SpawnProjectiles` (`KismetMathLibrary.MakeVector` _projectiletargetlocation_x_3 _projectiletargetlocation_y_3 _projectiletargetlocation_z_3) (`BlueprintGameplayTagLibrary.MakeLiteralGameplayTag` (struct :`TagName` "CombatSocket.ArrowsLeft")) false 0.0 (`self.MouseHitActor`))
                  (`self.SpawnProjectiles` (`KismetMathLibrary.MakeVector` _projectiletargetlocation_x _projectiletargetlocation_y _projectiletargetlocation_z) (`BlueprintGameplayTagLibrary.MakeLiteralGameplayTag` (struct :`TagName` "CombatSocket.ArrowsRight")) false 0.0 (`self.MouseHitActor`)))))
            (:`OnCompleted`
              (`self.K2_EndAbility` :!label _label))
            (:`OnInterrupted`
              (goto _label))
            (:`OnCancelled`
              (goto _label))))))))

(fn `SetRotaion`
  (params (Object :type "Object Object Reference"))
  (bind _aschakra_character (cast `ChakraCharacter` Object))
  (bind (_returnvalue_roll _returnvalue_pitch) (`KismetMathLibrary.BreakRotator` (`Actor.K2_GetActorRotation` _aschakra_character)))
  (bind (_returnvalue_roll_2 _returnvalue_pitch_2 _returnvalue_yaw) (`KismetMathLibrary.BreakRotator` (`KismetMathLibrary.Conv_VectorToRotator` (`KismetMathLibrary.GetDirectionUnitVector` (`Actor.K2_GetActorLocation` _aschakra_character) (`self.ProjectileTargetLocation`)))))
  (`Actor.K2_SetActorRotation` _aschakra_character (`KismetMathLibrary.MakeRotator` _returnvalue_roll _returnvalue_pitch _returnvalue_yaw) false))
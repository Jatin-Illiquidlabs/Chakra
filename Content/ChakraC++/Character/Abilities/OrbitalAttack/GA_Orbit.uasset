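; GA_Orbit is a Gameplay Ability that fires projectiles from the character's weapon socket toward the point under the mouse.
; It commits, waits for an input press, caches the cursor's hit location and actor, then plays Shakti's ability-two montage.
; On the FireBlast montage event, it yaws the character toward the target and calls SpawnProjectiles with a fixed target height and the hit actor as homing target.
; The montage finishing or being interrupted ends the ability.
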(event `self.K2_ActivateAbility`
  (bind (_projectiletargetlocation_x _projectiletargetlocation_y) (`KismetMathLibrary.BreakVector` (`self.ProjectileTargetLocation`)))
  (`self.K2_CommitAbility`)
  (`AbilityTask_WaitInputPress.WaitInputPress` false
    (:`OnPress`
      (bind (_asynctaskproxy _datahandle) (`TargetDataUnderMouse.CreateTargetDataUnderMouse`)
        (:`ValidData`
          (bind (_bblockinghit _binitialoverlap _time _distance _location _impactpoint _normal _impactnormal _physmat _hitactor) (`GameplayStatics.BreakHitResult` (`AbilitySystemBlueprintLibrary.GetHitResultFromTargetData` _datahandle)))
          (set `self.ProjectileTargetLocation` (`KismetMathLibrary.MakeVector` (.x _location) (.y _location) (.z _location)))
          (set `self.MouseHitActor` _hitactor)
          (`AbilityTask_PlayMontageAndWait.CreatePlayMontageAndWaitProxy` "None" "/Game/Characters/RevizedAnimations/ShaktiAnims/Shakti_AbilityTwoMobtage.Shakti_AbilityTwoMobtage" 1.0 "None" false
            (:`then`
              (`AbilityTask_WaitGameplayEvent.WaitGameplayEvent` (struct :`TagName` "Event.Montage.FireBlast") null
                (:`EventReceived`
                  (`self.SetRotaion` (`self.GetAvatarActorFromActorInfo`))
                  (`self.SpawnProjectiles` (`KismetMathLibrary.MakeVector` _projectiletargetlocation_x _projectiletargetlocation_y 45.0) (`BlueprintGameplayTagLibrary.MakeLiteralGameplayTag` (struct :`TagName` "CombatSocket.Weapon")) false 0.0 (`self.MouseHitActor`)))))
            (:`OnCompleted`
              (`self.K2_EndAbility` :!label _label))
            (:`OnBlendOut`
              (goto _label))
            (:`OnInterrupted`
              (goto _label))
            (:`OnCancelled`
              (goto _label))))))))

(fn `SetRotaion`
  (params (Object :type "Object Object Reference"))
  (bind _aschakra_character (cast `ChakraCharacter` Object))
  (bind (_returnvalue_roll _returnvalue_pitch) (`KismetMathLibrary.BreakRotator` (`Actor.K2_GetActorRotation` _aschakra_character)))
  (bind (_returnvalue_roll_2 _returnvalue_pitch_2 _returnvalue_yaw) (`KismetMathLibrary.BreakRotator` (`KismetMathLibrary.Conv_VectorToRotator` (`KismetMathLibrary.GetDirectionUnitVector` (`Actor.K2_GetActorLocation` _aschakra_character) (`self.ProjectileTargetLocation`)))))
  (`Actor.K2_SetActorRotation` _aschakra_character (`KismetMathLibrary.MakeRotator` _returnvalue_roll _returnvalue_pitch _returnvalue_yaw) false))
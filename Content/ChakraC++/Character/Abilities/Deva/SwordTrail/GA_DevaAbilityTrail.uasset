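; Gameplay ability for Deva's sword trail attack, aimed at the point under the mouse.
; On activation it commits, stores the hit location and actor from target data, turns the avatar toward that location and plays the AbilityThree montage.
; The montage's FireBolt gameplay event triggers SpawnTrail at that location and ends the ability without stopping the montage.
; Montage completion, blend-out, interruption or cancellation also ends it.
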(event `self.K2_ActivateAbility`
  (`self.K2_CommitAbility`)
  (bind (_asynctaskproxy _datahandle) (`TargetDataUnderMouse.CreateTargetDataUnderMouse`)
    (:`ValidData`
      (bind (_bblockinghit _binitialoverlap _time _distance _location _impactpoint _normal _impactnormal _physmat _hitactor) (`GameplayStatics.BreakHitResult` (`AbilitySystemBlueprintLibrary.GetHitResultFromTargetData` _datahandle)))
      (set `self.ProjectileTargetLocation` _location)
      (set `self.MouseHitActor` _hitactor)
      (message `CombatInterface.UpdateFacingTarget` (`self.GetAvatarActorFromActorInfo`) (`self.ProjectileTargetLocation`))
      (`AbilityTask_PlayMontageAndWait.CreatePlayMontageAndWaitProxy` "None" "/Game/Characters/RevizedAnimations/DevaAnims/Deva_AbilityThreeMontage.Deva_AbilityThreeMontage" 1.0 "None" false
        (:`then`
          (`AbilityTask_WaitGameplayEvent.WaitGameplayEvent` (struct :`TagName` "Event.Montage.FireBolt") null
            (:`EventReceived`
              (`self.SpawnTrail` (`self.ProjectileTargetLocation`))
              (`self.K2_EndAbility`))))
        (:`OnCompleted`
          (`self.K2_EndAbility` :!label _label))
        (:`OnBlendOut`
          (goto _label))
        (:`OnInterrupted`
          (goto _label))
        (:`OnCancelled`
          (goto _label))))))
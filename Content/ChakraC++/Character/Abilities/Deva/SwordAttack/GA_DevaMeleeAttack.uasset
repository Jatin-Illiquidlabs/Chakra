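; Gameplay ability for Deva's melee attack, which turns the character toward living BP_Zombie actors within close range and plays a random tagged attack montage.
; A trail cue runs during the swing, and the montage's tagged event triggers a sphere query at the matching combat socket, drawn for debugging.
; Non-friendly actors found take damage and show blood, a hit fires a melee impact cue, then the ability ends.
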(event `self.K2_ActivateAbility`
  (bind _returnvalue (`self.GetAvatarActorFromActorInfo`))
  (bind _returnvalue_2 (`self.GetAvatarActorFromActorInfo`))
  (bind _combatsocketlocation (`self.CombatSocketLocation`))
  (set `self.HasHitTarget` false)
  (bind _outactors (`GameplayStatics.GetAllActorsOfClass` "/Game/ChakraC++/Enemy/Zombie/BP_Zombie.BP_Zombie_C"))
  (for _array_element _outactors
    (if (and (< (`Actor.GetDistanceTo` _array_element _returnvalue) 300.0) (not (`ChakraCharacterBase.bDead` _array_element)))
      (`/Engine/EditorBlueprintResources/StandardMacros.IsValid` _array_element
        (:`Is Valid`
          (message `CombatInterface.UpdateFacingTarget` _returnvalue (`Actor.K2_GetActorLocation` _array_element))
          (bind _returnvalue_3 (message `CombatInterface.GetAttackMontages` (`self.GetAvatarActorFromActorInfo`)))
          (bind _output_get (set `self.TaggedMontage` (`self.GetRandomTaggedMontageFromArray` _returnvalue_3)))
          (`self.K2_AddGameplayCue` (struct :`TagName` "GameplayCue.Trail"))
          (bind (_montage _montagetag _sockettag) (break `TaggedMontage` _output_get))
          (`AbilityTask_PlayMontageAndWait.CreatePlayMontageAndWaitProxy` "None" _montage 1.0 "None" false
            (:`then`
              (`AbilityTask_WaitGameplayEvent.WaitGameplayEvent` _montagetag null
                (:`EventReceived`
                  (bind _returnvalue_4 (message `CombatInterface.GetCombatSocketLocation` _returnvalue_2 _sockettag))
                  (set `self.CombatSocketLocation` _returnvalue_4)
                  (bind _outoverlappingactors (`ChakraAbilitySystemLibrary.GetLivePlayersWithinRadius` _returnvalue_2 (`|MakeArray` _returnvalue_2) 45.0 _combatsocketlocation))
                  (`KismetSystemLibrary.DrawDebugSphere` _combatsocketlocation 70.0 12 (struct :`R` 0.120818 :`B` 1.0 :`A` 1.0) 2.0 2.0)
                  (for _array_element_2 _outoverlappingactors
                    (if (`ChakraAbilitySystemLibrary.IsNotFriend` _array_element_2 (`self.GetAvatarActorFromActorInfo`))
                      (`ChakraAbilitySystemLibrary.ApplyDamageEffect` (`self.MakeDamageEffectParamsFromClassDefaults` _array_element_2))
                      (set `self.HasHitTarget` true)
                      (message `CombatInterface.GetBloodEffect` _array_element_2)))
                  (if (`self.HasHitTarget`)
                    (bind _returnvalue_5 (message `EnemyInterface.GetCombatTarget` (`self.GetAvatarActorFromActorInfo`)))
                    (`self.K2_ExecuteGameplayCueWithParams` (struct :`TagName` "GameplayCue.MeleeImpact") (`AbilitySystemBlueprintLibrary.MakeGameplayCueParameters` 0.0 0.0 (struct) (struct) (struct) (`BlueprintGameplayTagLibrary.MakeGameplayTagContainerFromTag` (`.MontageTag` (break `TaggedMontage` (`self.TaggedMontage`)))) (struct) (`self.CombatSocketLocation`) (0.0 0.0 0.0) null (`self.GetAvatarActorFromActorInfo`) _returnvalue_5)))
                  (`self.K2_EndAbility`))))
            (:`OnCancelled`
              (`self.K2_EndAbility`))))))))
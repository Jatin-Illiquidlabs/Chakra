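; Deva's teleport gameplay ability, which throws a sword projectile or, if one already exists, teleports the avatar to it.
; It gets the point under the mouse, waits briefly, then searches the world for a sword projectile.
; If found, it teleports there and destroys the projectile.
; Otherwise it faces the target, plays a montage and launches the projectile from the weapon socket on the FireBolt event.
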(event `self.K2_ActivateAbility`
  (`self.K2_CommitAbility`)
  (bind (_asynctaskproxy _datahandle) (`TargetDataUnderMouse.CreateTargetDataUnderMouse`)
    (:`ValidData`
      (bind (_bblockinghit _binitialoverlap _time _distance _location _impactpoint _normal _impactnormal _physmat _hitactor) (`GameplayStatics.BreakHitResult` (`AbilitySystemBlueprintLibrary.GetHitResultFromTargetData` _datahandle)))
      (set `self.ProjectileTargetLocation` _location)
      (set `self.MouseHitActor` _hitactor)
      (`KismetSystemLibrary.Delay` 0.2)
      (bind _returnvalue (`GameplayStatics.GetActorOfClass` "/Game/ChakraC++/Character/Abilities/Deva/Teleport/SwordTeleportProjectile_BP.SwordTeleportProjectile_BP_C"))
      (`/Engine/EditorBlueprintResources/StandardMacros.IsValid` _returnvalue
        (:`Is Valid`
          (`Actor.K2_TeleportTo` :`self` (`self.GetAvatarActorFromActorInfo`) :`DestLocation` (`Actor.K2_GetActorLocation` _returnvalue))
          (`Actor.K2_DestroyActor` _returnvalue)
          (message `CombatInterface.UpdateFacingTarget` (`self.GetAvatarActorFromActorInfo`) (`self.ProjectileTargetLocation`))
          (set `self.IsValid` false)
          (`self.K2_EndAbility`))
        (:`Is Not Valid`
          (message `CombatInterface.UpdateFacingTarget` (`self.GetAvatarActorFromActorInfo`) (`self.ProjectileTargetLocation`))
          (`AbilityTask_PlayMontageAndWait.CreatePlayMontageAndWaitProxy` "None" "/Game/Characters/RevizedAnimations/DevaAnims/Deva_AbilityOneMontage.Deva_AbilityOneMontage" 1.0 "None" false
            (:`then`
              (`AbilityTask_WaitGameplayEvent.WaitGameplayEvent` (struct :`TagName` "Event.Montage.FireBolt") null
                (:`EventReceived`
                  (`self.ProjectileAttack` (`self.ProjectileTargetLocation`) (`BlueprintGameplayTagLibrary.MakeLiteralGameplayTag` (struct :`TagName` "CombatSocket.Weapon")))
                  (set `self.IsValid` true)
                  (`self.K2_EndAbility`))))
            (:`OnCompleted`
              (`self.K2_EndAbility` :!label _label))
            (:`OnBlendOut`
              (goto _label))
            (:`OnInterrupted`
              (goto _label))
            (:`OnCancelled`
              (goto _label))))))))

(event `self.K2_OnEndAbility`
  (params (bWasCancelled :type Boolean)))
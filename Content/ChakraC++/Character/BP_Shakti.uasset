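; BP_Shakti is a character Blueprint that adds motion-warp facing and fixed graphics settings on top of its parent class.
; UpdateFacingTarget writes the given location to the "FacingTarget" warp target on the MotionWarping component.
; BeginPlay calls the parent, then overwrites and applies game-wide scalability settings at mostly low levels, a side effect of spawning this character.
; Tick only forwards to the parent, and the construction script is empty.
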(event `CombatInterface.UpdateFacingTarget`
  (params (Target :type "Vector Structure (by ref)"))
  (`MotionWarpingComponent.AddOrUpdateWarpTargetFromLocation` (`self.MotionWarping`) "FacingTarget" Target))

(event `self.ReceiveBeginPlay`
  (`parent.ReceiveBeginPlay`)
  (bind _returnvalue (`GameUserSettings.GetGameUserSettings`))
  (`GameUserSettings.SetTextureQuality` _returnvalue 1)
  (`GameUserSettings.SetVisualEffectQuality` _returnvalue 0)
  (`GameUserSettings.SetAntiAliasingQuality` _returnvalue 2)
  (`GameUserSettings.SetViewDistanceQuality` _returnvalue 1)
  (`GameUserSettings.SetPostProcessingQuality` _returnvalue 0)
  (`GameUserSettings.SetShadowQuality` _returnvalue 0)
  (`GameUserSettings.ApplySettings` _returnvalue false))

(event `self.ReceiveTick`
  (params (DeltaSeconds :type "Float (single-precision)"))
  (`parent.ReceiveTick` DeltaSeconds))

(fn `UserConstructionScript`)
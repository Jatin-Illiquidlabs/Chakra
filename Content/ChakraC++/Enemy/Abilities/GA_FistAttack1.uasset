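; Enemy gameplay ability that, despite its FistAttack name, transforms a Zombie-type Chakra enemy into a werewolf.
; After committing, it plays the transformation montage for Zombies and ends immediately for other character types.
; An Effects.HitReact gameplay event received during the montage swaps the skeletal mesh to the werewolf and ends the ability, without stopping the montage.
; Montage completion, interruption or cancellation also ends it.
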(event `self.K2_ActivateAbility`
  (`self.K2_CommitAbility`)
  (bind _aschakra_enemy_character (cast `ChakraEnemyCharacter` (`self.GetAvatarActorFromActorInfo`)))
  (if (`|EnumEquality` (`ChakraEnemyCharacter.CharacterType` _aschakra_enemy_character) "Zombie")
    (`AbilityTask_PlayMontageAndWait.CreatePlayMontageAndWaitProxy` "None" "/Game/Characters/RevizedAnimations/ZombieAnims/Tranformation_Anims.Tranformation_Anims" 1.1 "None" false
      (:`then`
        (`AbilityTask_WaitGameplayEvent.WaitGameplayEvent` (struct :`TagName` "Effects.HitReact") null
          (:`EventReceived`
            (bind _aschakra_enemy_character_2 (cast `ChakraEnemyCharacter` (`self.GetAvatarActorFromActorInfo`)))
            (`SkeletalMeshComponent.SetSkeletalMeshAsset` (`Character.Mesh` _aschakra_enemy_character_2) "/Game/Characters/WareWolf_Enemy/Ware_Waolf_Enemy.Ware_Waolf_Enemy")
            (`self.K2_EndAbility`))))
      (:`OnCompleted`
        (`self.K2_EndAbility` :!label _label))
      (:`OnInterrupted`
        (goto _label))
      (:`OnCancelled`
        (goto _label)))
    (else
      (goto _label))))
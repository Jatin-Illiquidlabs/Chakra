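; Base enemy Blueprint that handles spawn scaling, facing warps and dissolve visuals.
; On BeginPlay a timeline drives the mesh's uniform relative scale.
; UpdateFacingTarget feeds a location to Motion Warping as the FacingTarget warp target.
; Two dissolve events, one named for the weapon, each play their own timeline to animate the Dissolve parameter on the dynamic material instance passed in.
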(event `self.ReceiveBeginPlay`
  (bind (_direction _scaletrack) (`Timeline|Timeline_1`)
    (:`Update`
      (`SceneComponent.SetRelativeScale3D` (`self.Mesh`) (`KismetMathLibrary.MakeVector` _scaletrack _scaletrack _scaletrack)))))

(event `CombatInterface.UpdateFacingTarget`
  (params (Target :type "Vector Structure (by ref)"))
  (`MotionWarpingComponent.AddOrUpdateWarpTargetFromLocation` (`self.MotionWarping1`) "FacingTarget" Target))

(event `self.StartDissolveTimeline`
  (params (DynamicMaterialInstance :type "MaterialInstanceDynamic Object Reference"))
  (bind (_direction _dissolve_track) (`Timeline|Timeline`)
    (:`Update`
      (`MaterialInstanceDynamic.SetScalarParameterValue` DynamicMaterialInstance "Dissolve" _dissolve_track))))

(event `self.StartWeaponDissolveTimeline`
  (params (DynamicMaterialInstance :type "MaterialInstanceDynamic Object Reference"))
  (bind (_direction _dissolve_track) (`Timeline|Timeline_0`)
    (:`Update`
      (`MaterialInstanceDynamic.SetScalarParameterValue` DynamicMaterialInstance "Dissolve" _dissolve_track))))

(fn `UserConstructionScript`)
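; Spell actor that spawns a ring of orbiting Niagara tornado effects and destroys itself after a set lifetime.
; BeginPlay adds one Niagara component per tornado to an array, then waits before destroying the actor.
; Tick repositions each component with evenly phased sine and cosine offsets around the actor, while a second time-based sine pulses the radius through the center.
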(event `self.ReceiveTick`
  (params (DeltaSeconds :type "Float (single-precision)"))
  (bind _returnvalue (* (`KismetMathLibrary.GetPI`) 2.0))
  (bind _returnvalue_2 (* (`KismetSystemLibrary.GetGameTimeInSeconds`) _returnvalue))
  (bind _returnvalue_3 (* (`self.CircleRadius`) (`KismetMathLibrary.Sin` (/ _returnvalue_2 (`self.CircleRipleTime`)))))
  (for (_array_element _array_index) (`self.Tornados`)
    (bind _returnvalue_4 (+ (* (/ (`KismetMathLibrary.Conv_IntToDouble` _array_index) (`KismetMathLibrary.Conv_ByteToDouble` (`self.NumberOfTornado`))) _returnvalue) (/ _returnvalue_2 (`self.CircleMovingTime`))))
    (`SceneComponent.K2_SetRelativeLocation` _array_element (`KismetMathLibrary.MakeVector` (* (`KismetMathLibrary.Sin` _returnvalue_4) _returnvalue_3) (* (`KismetMathLibrary.Cos` _returnvalue_4) _returnvalue_3) 1.0) false false)))

(event `self.ReceiveBeginPlay`
  (for _ (range 1 (+ (`KismetMathLibrary.Conv_ByteToInt` (`self.NumberOfTornado`)) 1))
    (bind _returnvalue (`AddComponent|NODE_AddNiagaraComponent-0`))
    (`KismetArrayLibrary.Array_Add` (`self.Tornados`) _returnvalue))
  (`KismetSystemLibrary.Delay` (`self.TimeToDestroyActor`))
  (`self.K2_DestroyActor`))

(fn `UserConstructionScript`)